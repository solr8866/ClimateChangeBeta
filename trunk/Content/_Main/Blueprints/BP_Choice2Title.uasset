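; BP_Choice2Title is an actor that shows a title text during the second choice step of the VR game.
; It hides the title on BeginPlay and binds to the VRGameMode's 07Choice2 and 07Choice2Done events.
; When the choice starts, it shows the title and plays a timeline that animates the text render color, and when the choice is done it hides the title again.
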(event `self.ReceiveBeginPlay`
  (`SceneComponent.SetVisibility` (`self.Title`) false false)
  (bind _asvrgame_mode (cast `/Game/_Main/Blueprints/VRGameMode` (`GameplayStatics.GetGameMode`)))
  (add `/Game/_Main/Blueprints/VRGameMode.07_Choice_2` _asvrgame_mode (delegate `Choice2Start`))
  (add `/Game/_Main/Blueprints/VRGameMode.07_Choice_2Done` _asvrgame_mode (delegate `Choice2Done`)))

(event `Choice2Done`
  (`SceneComponent.SetVisibility` (`self.Title`) false false))

(event `Choice2Start`
  (`SceneComponent.SetVisibility` (`self.Title`) true false)
  (bind (_direction _color) (`Timeline|Timeline_0`)
    (:`Update`
      (`TextRenderComponent.SetTextRenderColor` (`self.Title`) (`KismetMathLibrary.Conv_LinearColorToColor` _color)))))

(fn `UserConstructionScript`)