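; Base actor for one answer option in a two-option VR choice, shown and hidden by VRGameMode events.
; ToggleParticle refreshes a countdown that Tick uses to show attraction particles, and spawns a camera-facing progress bar.
; If the countdown lapses, Tick cancels the bar.
; When the bar finishes, the option text turns green or red by IsRightAnswer, then after a short delay notifies the game mode.
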(event `self.ReceiveBeginPlay`
  (`SceneComponent.SetVisibility` (`self.Option`) false false)
  (`SceneComponent.SetVisibility` (`self.P_GPU_particles_attraction`) false false)
  (set `self.bIsChoiceStart` false)
  (bind _asvrgame_mode (cast `/Game/_Main/Blueprints/VRGameMode` (`GameplayStatics.GetGameMode`)))
  (add `/Game/_Main/Blueprints/VRGameMode.07_Choice_2Done` _asvrgame_mode (delegate `Choice_2Done`))
  (add `/Game/_Main/Blueprints/VRGameMode.07_Choice_2` _asvrgame_mode (delegate `FadeOutText`)))

(event `Choice_2Done`
  (`self.Show Option` false)
  (`self.Show Particles` false))

(event `FadeOutText`
  (`self.Show Option` true))

(event `ToggleParticle`
  (params (bIsParticleOpen :type Boolean))
  (if (and bIsParticleOpen (`self.bIsChoiceStart`))
    (set `self.ParticleOpenCountDown` (`self.ParticleOpenDuration`))
    (`/Engine/EditorBlueprintResources/StandardMacros.IsValid` (`self.ProgressBar`)
      (:`Is Not Valid`
        (bind _asmotion_controller_pawn (cast `/Game/VirtualRealityBP/Blueprints/MotionControllerPawn` (`GameplayStatics.GetPlayerPawn` 0)))
        (bind (_location _rotation) (`self.LocationAndRotation` _asmotion_controller_pawn (`self.K2_GetActorLocation`)))
        (bind _returnvalue (`|SpawnActorFromClass` "/Game/AVRFramework/Blueprints/UI/ProgressBar/BP_ProgressBar.BP_ProgressBar_C" (`KismetMathLibrary.MakeTransform` _location _rotation) "Undefined" "OverrideRootScale" null 0.0 10.0 null))
        (bind _output_get (set `self.ProgressBar` _returnvalue))
        (add `/Game/AVRFramework/Blueprints/UI/ProgressBar/BP_ProgressBar.Finished` _output_get (delegate `ProgressBarFinished`))
        (`/Game/AVRFramework/Blueprints/UI/ProgressBar/BP_ProgressBar.PlayProgressBar` (`self.ProgressBar`) 2.0)))))

(event `ProgressBarFinished`
  (bind _option (`self.Option`))
  (remove `/Game/AVRFramework/Blueprints/UI/ProgressBar/BP_ProgressBar.Finished` (stale `ToggleParticle` _output_get) (delegate `ProgressBarFinished`))
  (message `/Game/AVRFramework/Interface/Interface_Deleteable.Delete` (`self.ProgressBar`) "NewEnumerator1")
  (set `self.ProgressBar` null)
  (set `self.bIsChoiceStart` false)
  (if (`self.bIsRightAnswer`)
    (`TextRenderComponent.SetTextRenderColor` _option (`KismetMathLibrary.Conv_LinearColorToColor` (struct :`G` 1.0 :`A` 1.0)))
    (else
      (`TextRenderComponent.SetTextRenderColor` _option (`KismetMathLibrary.Conv_LinearColorToColor` (struct :`R` 1.0 :`A` 1.0)))))
  (`KismetSystemLibrary.Delay` 0.5)
  (bind _asvrgame_mode (cast `/Game/_Main/Blueprints/VRGameMode` (`GameplayStatics.GetGameMode`)))
  (`/Game/_Main/Blueprints/VRGameMode.CBE_Choice_2` _asvrgame_mode))

(event `self.ReceiveTick`
  (params (DeltaSeconds :type "Float (single-precision)"))
  (bind _returnvalue (> (`self.ParticleOpenCountDown`) 0.0))
  (if (`self.bIsChoiceStart`)
    (if _returnvalue
      (`self.Show Particles` _returnvalue)
      (else
        (`/Engine/EditorBlueprintResources/StandardMacros.IsValid` (`self.ProgressBar`)
          (:`Is Valid`
            (message `/Game/AVRFramework/Interface/Interface_Deleteable.Delete` (`self.ProgressBar`) "NewEnumerator1")
            (set `self.ProgressBar` null)
            (`self.Show Particles` false)))))
    (set `self.ParticleOpenCountDown` (- (`self.ParticleOpenCountDown`) DeltaSeconds))))

(fn `Show Option`
  (params (bIsShowOption :type Boolean))
  (`SceneComponent.SetVisibility` (`self.Option`) bIsShowOption false)
  (set `self.bIsChoiceStart` bIsShowOption))

(fn `Show Particles`
  (params (bIsVisibility :type Boolean))
  (`SceneComponent.SetVisibility` (`self.P_GPU_particles_attraction`) bIsVisibility false))

(fn `UserConstructionScript`)