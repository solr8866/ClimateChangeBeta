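; BP_Choice1 is a VR choice display showing a title, three text options and an attraction particle effect, all hidden at start.
; It binds to two VRGameMode story events: the first choice event reveals everything and animates text color through a timeline.
; After a delay, Option1, Option3 and the particles hide, leaving Option2 and the title.
; The later flies-come event hides those two shortly afterward.
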(event `self.ReceiveBeginPlay`
  (`SceneComponent.SetVisibility` (`self.Option1`) false false)
  (`SceneComponent.SetVisibility` (`self.Option2`) false false)
  (`SceneComponent.SetVisibility` (`self.Option3`) false false)
  (`SceneComponent.SetVisibility` (`self.Title`) false false)
  (`SceneComponent.SetVisibility` (`self.P_GPU_particles_attraction`) false false)
  (bind _asvrgame_mode (cast `/Game/_Main/Blueprints/VRGameMode` (`GameplayStatics.GetGameMode`)))
  (add `/Game/_Main/Blueprints/VRGameMode.02_Choice_1` _asvrgame_mode (delegate `FadeOutText`))
  (add `/Game/_Main/Blueprints/VRGameMode.03_FilesCome` _asvrgame_mode (delegate `FliesCome`)))

(event `FliesCome`
  (`KismetSystemLibrary.Delay` 1.0)
  (`SceneComponent.SetVisibility` (`self.Option2`) false false)
  (`SceneComponent.SetVisibility` (`self.Title`) false false))

(event `FadeOutText`
  (`SceneComponent.SetVisibility` (`self.Option1`) true false)
  (`SceneComponent.SetVisibility` (`self.Option2`) true false)
  (`SceneComponent.SetVisibility` (`self.Option3`) true false)
  (`SceneComponent.SetVisibility` (`self.Title`) true false)
  (`SceneComponent.SetVisibility` (`self.P_GPU_particles_attraction`) true false)
  (bind (_direction _color) (`Timeline|Timeline_0`)
    (:`Update`
      (`TextRenderComponent.SetTextRenderColor` (`self.Option1`) (`KismetMathLibrary.Conv_LinearColorToColor` _color))
      (`TextRenderComponent.SetTextRenderColor` (`self.Option2`) (`KismetMathLibrary.Conv_LinearColorToColor` _color))
      (`TextRenderComponent.SetTextRenderColor` (`self.Option3`) (`KismetMathLibrary.Conv_LinearColorToColor` _color))
      (`TextRenderComponent.SetTextRenderColor` (`self.Title`) (`KismetMathLibrary.Conv_LinearColorToColor` _color))
      (`KismetSystemLibrary.Delay` 8.0)
      (`SceneComponent.SetVisibility` (`self.Option1`) false false)
      (`SceneComponent.SetVisibility` (`self.P_GPU_particles_attraction`) false false)
      (`SceneComponent.SetVisibility` (`self.Option3`) false false))))

(fn `UserConstructionScript`)