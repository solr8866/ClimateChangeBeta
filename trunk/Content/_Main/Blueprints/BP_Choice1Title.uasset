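; BP_Choice1Title is an actor that shows a text title during the first choice moment in the VR game.
; It starts hidden and binds to the 02Choice1 and 02Choice1Done events on VRGameMode.
; The choice event reveals the title and plays a timeline that animates its text render color.
; The done event hides it again.
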(event `self.ReceiveBeginPlay`
  (`SceneComponent.SetVisibility` (`self.Title`) false false)
  (bind _asvrgame_mode (cast `/Game/_Main/Blueprints/VRGameMode` (`GameplayStatics.GetGameMode`)))
  (add `/Game/_Main/Blueprints/VRGameMode.02_Choice_1` _asvrgame_mode (delegate `FadeOutText`))
  (add `/Game/_Main/Blueprints/VRGameMode.02_Choice_1Done` _asvrgame_mode (delegate `FliesCome`)))

(event `FliesCome`
  (`SceneComponent.SetVisibility` (`self.Title`) false false))

(event `FadeOutText`
  (`SceneComponent.SetVisibility` (`self.Title`) true false)
  (bind (_direction _color) (`Timeline|Timeline_1`)
    (:`Update`
      (`TextRenderComponent.SetTextRenderColor` (`self.Title`) (`KismetMathLibrary.Conv_LinearColorToColor` _color)))))

(fn `UserConstructionScript`)