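; VR game mode that runs a three-act narrated caribou story, moving from intro through two right-or-wrong choices to an ending.
; BeginPlay enables the HMD, plays the intro and binds both choice callbacks, whose answers select the voice-over and advance the acts.
; Act 2 plays a level sequence whose events cue snow, migration, melting, flies and the second choice through numbered Call functions.
; Timelines tint the booth through a material parameter collection, and Act 3 opens baby caribou media.
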(event `Choice1Done` :!signature `self.CBE_Choice_1`
  (params (bIsRightAnswer :type Boolean))
  (bind _vo01_choice1right (`self.VO01_Choice1Right`))
  (bind _vo01_choice1wrong (`self.VO01_Choice1Wrong`))
  ;[1 1 1] ACT 1_Choice1
  (`self.02_Choice_1Done`)
  (`|ExecutionSequence`
    (:`then_0`
      (`AudioComponent.FadeOut` (`self.Music`) 2.0 0.0 "Linear")
      (`KismetSystemLibrary.Delay` 2.0)
      (`AudioComponent.SetPaused` (`self.Music`) true))
    (:`then_1`
      (bind (_direction _basecolor) (`Timeline|AdjustBoothColor` :!via `ReverseFromEnd`)
        (:`Update`
          (`KismetMaterialLibrary.SetVectorParameterValue` "/Game/_Main/Meshes/Booth/MC_Booth.MC_Booth" "BoothColor" _basecolor))))
    (:`then_2`
      (if bIsRightAnswer
        (`self.PlayVO` _vo01_choice1right)
        (`KismetSystemLibrary.Delay` (`SoundBase.Duration` _vo01_choice1right))
        (else
          (`self.PlayVO` _vo01_choice1wrong)
          (`KismetSystemLibrary.Delay` (`SoundBase.Duration` _vo01_choice1wrong))))
      (`self.ACT2Start`))))

(event `self.ReceiveBeginPlay`
  (bind _vo01_choice1 (`self.VO01_Choice1`))
  (`HeadMountedDisplayFunctionLibrary.EnableHMD` true)
  (`KismetSystemLibrary.ExecuteConsoleCommand` "fullscreen" null)
  ;[1 1 1] Introduction
  (`AudioComponent.Play` (`self.Music`) 0.0)
  (`PlayerCameraManager.StartCameraFade` :`self` (`GameplayStatics.GetPlayerCameraManager` 0) :`ToAlpha` 1.0 :`Duration` (`self.FadeOutDuration`) :`bHoldWhenFinished` true)
  (`KismetSystemLibrary.Delay` 8.0)
  (`PlayerCameraManager.StartCameraFade` :`self` (`GameplayStatics.GetPlayerCameraManager` 0) :`FromAlpha` 1.0 :`Duration` (`self.FadeInDuration`) :`bHoldWhenFinished` true)
  (`KismetSystemLibrary.Delay` 2.0)
  (`self.PlayVO` _vo01_choice1)
  (`KismetSystemLibrary.Delay` (`SoundBase.Duration` _vo01_choice1))
  (`|ExecutionSequence`
    (:`then_0`
      ;[1 1 1] ACT 1_Choice1
      (bind (_direction _basecolor) (`Timeline|Timeline_1`)
        (:`Update`
          (`KismetMaterialLibrary.SetVectorParameterValue` "/Game/_Main/Meshes/Booth/MC_Booth.MC_Booth" "BoothColor" _basecolor)
          (`self.02_Choice_1`)
          (add `self.CBE_Choice_1` (delegate `Choice1Done`)))))
    (:`then_1`
      (add `self.CBE_Choice_2` (delegate `CBE_Choice2Making`)))))

(event `CBE_Choice2Making` :!signature `self.CBE_Choice_2`
  (params (bIsRightAnswer :type Boolean))
  (`self.Act3Start` bIsRightAnswer))

(event `ACT2Start`
  ;[1 1 1] ACT 2
  (`MovieSceneSequencePlayer.Play` (`ActorSequenceComponent.SequencePlayer` (`self.VO02_Choice2Sequence`))))

(event `ACT3Start`
  (params (bIsRightAnswer :type Boolean))
  (bind _vo02_choice2wrong (`self.VO02_Choice2Wrong`))
  (bind _vo02_choice2right (`self.VO02_Choice2Right`))
  (bind _vo03_ending_cue (`self.VO03_Ending_Cue`))
  (bind _music (`self.Music`))
  ;[1 1 1] Choice2 + ACT 3
  (`self.07_Choice_2Done`)
  (`|ExecutionSequence`
    (:`then_1`
      (if bIsRightAnswer
        (`self.PlayVO` _vo02_choice2right)
        (`KismetSystemLibrary.Delay` (`SoundBase.Duration` _vo02_choice2right))
        (else
          (`self.PlayVO` _vo02_choice2wrong)
          (`KismetSystemLibrary.Delay` (`SoundBase.Duration` _vo02_choice2wrong))))
      (`self.PlayVO` _vo03_ending_cue)
      (`KismetSystemLibrary.Delay` (`SoundBase.Duration` _vo03_ending_cue))
      (`AudioComponent.FadeOut` (`self.Music`) 2.0 0.0 "Linear")
      (`MediaPlayer.OpenSource` (`self.MediaPlayer`) "/Game/Movies/BabyCaribou_MediaSource.BabyCaribou_MediaSource")
      (`GameplayStatics.PlaySound2D` "/Game/_Main/Audios/BabyCaribou_Cue.BabyCaribou_Cue" 1.0 1.0 0.0 null null))
    (:`then_2`
      (`KismetSystemLibrary.Delay` 15.0)
      (`AudioComponent.SetPaused` _music false)
      (`AudioComponent.FadeIn` _music 2.0 0.6 59.0 "Linear")
      (`|ExecutionSequence`
        (:`then_0`
          (`KismetSystemLibrary.Delay` 2.0)
          (`self.06_FadeOut` :!label _label))
        (:`then_1`
          (bind (_direction _basecolor) (`Timeline|GoodNews`)
            (:`Update`
              (`KismetMaterialLibrary.SetVectorParameterValue` "/Game/_Main/Meshes/Booth/MC_Booth.MC_Booth" "BoothColor" _basecolor))
            (:`Finished`
              (goto _label))))))))

(event `FliesCome`
  (params (Owner :type "Actor Object Reference"))
  (`self.03_FilesCome`))

(event `Migration1`
  (params (Owner :type "Actor Object Reference"))
  (`|ExecutionSequence`
    (:`then_0`
      (bind _returnvalue (`GameplayStatics.SpawnEmitterAtLocation` "/Game/_Main/Snow/snow.Snow" (-50.0 30.0 700.0) (struct) (1.0 1.0 1.0) false))
      (set `self.SnowParticle` _returnvalue))
    (:`then_1`
      (bind (_direction _basecolor) (`Timeline|Timeline_0`)
        (:`Update`
          (`KismetMaterialLibrary.SetVectorParameterValue` "/Game/_Main/Meshes/Booth/MC_Booth.MC_Booth" "BoothColor" _basecolor))))
    (:`then_2`
      (`self.PlaySFX` (`self.CaribouRun`))
      (`self.04_Migration`))))

(event `StopSnowingStartMelting`
  (params (Owner :type "Actor Object Reference"))
  (`|ExecutionSequence`
    (:`then_0`
      (`ActorComponent.Deactivate` (`self.SnowParticle`))
      (`self.05_Glacier Melting`))
    (:`then_1`
      (bind (_direction _basecolor) (`Timeline|Timeline_3` :!via `ReverseFromEnd`)
        (:`Update`
          (`KismetMaterialLibrary.SetVectorParameterValue` "/Game/_Main/Meshes/Booth/MC_Booth.MC_Booth" "BoothColor" _basecolor))))))

(event `FliesComeAgain`
  (params (Owner :type "Actor Object Reference"))
  (`self.05_Flies Come Again`))

(event `FadeOut`
  (params (Owner :type "Actor Object Reference")))

(event `ShowChoice2`
  (params (Owner :type "Actor Object Reference"))
  (`self.07_Choice_2`))

(fn `PlaySFX`
  (params (SoundClip :type "SoundBase Object Reference"))
  (bind _sfx (`self.SFX`))
  (`AudioComponent.SetSound` _sfx SoundClip)
  (`AudioComponent.Play` _sfx 0.0))

(fn `PlayVO`
  (params (SoundClip :type "SoundBase Object Reference"))
  (bind _v_o_ (`self.V.O.`))
  (`AudioComponent.SetSound` _v_o_ SoundClip)
  (`AudioComponent.Play` _v_o_ 0.0))

(fn `UserConstructionScript`)