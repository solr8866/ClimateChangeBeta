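; BP_MComp is a base actor for VR motion controller components, with empty input and visibility hooks for children to override.
; On BeginPlay it registers with its parent BP_BaseMotionController and caches the hand side, pawn and controller.
; Tick converts thumbstick axes, zeroed while inactive, into raw and pawn-yaw-relative rotations.
; Haptic requests play curve timelines scaled to duration, sending amplitude with a per-HMD multiplier to the player controller.
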(event `self.ReceiveBeginPlay`
  ;[1 1 1] Setup
  (bind _asbp_base_motion_controller (cast `/Game/AVRFramework/Blueprints/VR/MotionControllers/BP_BaseMotionController` (`self.GetParentActor`)))
  (`BlueprintSetLibrary.Set_Add` (`/Game/AVRFramework/Blueprints/VR/MotionControllers/BP_BaseMotionController.AttachedMComps` _asbp_base_motion_controller) self)
  (`self.Setup` (`/Game/AVRFramework/Blueprints/VR/MotionControllers/BP_BaseMotionController.Side` _asbp_base_motion_controller) (`/Game/AVRFramework/Blueprints/VR/MotionControllers/BP_BaseMotionController.VRPawn` _asbp_base_motion_controller) (`/Game/AVRFramework/Blueprints/VR/MotionControllers/BP_BaseMotionController.MotionController` _asbp_base_motion_controller) _asbp_base_motion_controller)
  (`self.Interface_SetActive` (`self.Active`)))

(event `self.ReceiveTick`
  (params (DeltaSeconds :type "Float (single-precision)"))
  (bind _basemotioncontroller (`self.BaseMotionController`))
  ;[1 1 1] Constantly Update Thumbstick Values
  (`/Engine/EditorBlueprintResources/StandardMacros.IsValid` _basemotioncontroller
    (:`Is Valid`
      (`self.UpdateThumbstick` (`/Game/AVRFramework/Blueprints/VR/MotionControllers/BP_BaseMotionController.Axis_Thumbstick_Up` _basemotioncontroller) (`/Game/AVRFramework/Blueprints/VR/MotionControllers/BP_BaseMotionController.Aixs_Thumbstick_Right` _basemotioncontroller)))))

(event `self.Interface_SetActive`
  (params (Set :type Boolean))
  ;[1 1 1] Active Interface
  (set `self.Active` Set))

(event `self.Interface_ToggleActive`
  ;[1 1 1] Active Interface
  (bind _isactive (`self.Interface_IsActive`))
  (`self.Interface_SetActive` (not _isactive)))

(event `KeyInput`
  (params (Key :type "/Game/AVRFramework/Enums/Enum_MotionController_Buttons Enum" :default "NewEnumerator1") (Set :type Boolean))
  ;[1 1 1] Override KeyInput
)

(event `FunctionInput`
  (params (Function :type "/Game/AVRFramework/Enums/Enum_Control_Function Enum" :default "NewEnumerator0") (Set :type Boolean))
  ;[1 1 1] Override Function Input
)

(event `SetHaptics`
  (params (Curve :type "/Game/AVRFramework/Enums/Enum_Haptic_Curves Enum" :default "NewEnumerator4") (Duration :type "Float (double-precision)") (Strength :type "Float (double-precision)"))
  (bind _returnvalue (/ 1.0 Duration))
  ;[1 1 1] Haptics
  (if (== Duration 0.0)
    (`self.ExecuteHaptic` 0.01 1.0 Strength :!label _label)
    (else
      (switch `/Game/AVRFramework/Enums/Enum_Haptic_Curves` Curve
        (:`NewEnumerator4`
          (goto _label))
        (:`NewEnumerator0`
          (`TimelineComponent.SetPlayRate` (`self.HapticsTimelineConstant`) _returnvalue)
          (bind (_direction _percent) (`Timeline|HapticsTimelineConstant` :!via `PlayFromStart`)
            (:`Update`
              (`self.ExecuteHaptic` 0.01 _percent Strength))))
        (:`NewEnumerator1`
          (`TimelineComponent.SetPlayRate` (`self.HapticsTimelineUpCurve`) _returnvalue)
          (bind (_direction_2 _percent_2) (`Timeline|HapticsTimelineUpCurve` :!via `PlayFromStart`)
            (:`Update`
              (`self.ExecuteHaptic` 0.01 _percent_2 Strength))))
        (:`NewEnumerator2`
          (`TimelineComponent.SetPlayRate` (`self.HapticsTimelineDownCurve`) _returnvalue)
          (bind (_direction_3 _percent_3) (`Timeline|HapticsTimelineDownCurve` :!via `PlayFromStart`)
            (:`Update`
              (`self.ExecuteHaptic` 0.01 _percent_3 Strength))))
        (:`NewEnumerator3`
          (`TimelineComponent.SetPlayRate` (`self.HapticsTimelineNormalCurve`) _returnvalue)
          (bind (_direction_4 _percent_4) (`Timeline|HapticsTimelineNormalCurve` :!via `PlayFromStart`)
            (:`Update`
              (`self.ExecuteHaptic` 0.01 _percent_4 Strength))))))))

(event `ExecuteHaptic`
  (params (Frequency :type "Float (double-precision)" :default 0.01) (Amplitude :type "Float (double-precision)") (StengthMultiplyer :type "Float (double-precision)"))
  ;[1 1 1] Haptics
  (bind _infocontrols (`/Game/AVRFramework/Libraries/Lib_Core.getInfoControls` self))
  (bind _asbp_player_controller_main (cast `/Game/AVRFramework/Framework/BP_PlayerController_Main` (`Pawn.GetController` (`self.VRPawn`))))
  (`PlayerController.SetHapticsByValue` _asbp_player_controller_main Frequency (* Amplitude StengthMultiplyer (`BlueprintMapLibrary.Map_Find` (`/Game/AVRFramework/Blueprints/Info/BP_Info_Controls.HapticMultiplier` _infocontrols) (`/Game/AVRFramework/Blueprints/VR/MotionControllers/BP_BaseMotionController.HMD` (`self.BaseMotionController`)))) (select `/Game/AVRFramework/Enums/Enum_Side` (`self.Side`) :`NewEnumerator0` "Left" :`NewEnumerator1` "Right" :!type "EControllerHand Enum")))

(fn `getAllAttachedActors`
  (returns (Actors :type "Set of Actor Object Reference"))
  (return))

(fn `getRotationFromInput`
  (params (UpAxis :type "Float (double-precision)") (RightAxis :type "Float (double-precision)"))
  (returns (OutRotation :type "Rotator Structure") (NoOffsetOutRotation :type "Rotator Structure"))
  (bind _returnvalue (`KismetMathLibrary.Normal` (`KismetMathLibrary.MakeVector` UpAxis RightAxis)))
  (return (`KismetMathLibrary.Conv_VectorToRotator` (`KismetMathLibrary.GreaterGreater_VectorRotator` _returnvalue (`KismetMathLibrary.MakeRotator` 0.0 0.0 (.yaw (`self.K2_GetActorRotation` (`self.VRPawn`)))))) (`KismetMathLibrary.Conv_VectorToRotator` _returnvalue)))

(fn `Interface_IsActive`
  (returns (IsActive :type Boolean))
  (return (`self.Active`)))

(fn `Setup`
  (params (Side :type "/Game/AVRFramework/Enums/Enum_Side Enum" :default "NewEnumerator0") (VRPawn :type "/Game/AVRFramework/Framework/BP_Pawn_VR Object Reference") (MotionComponent :type "MotionControllerComponent Object Reference") (MotionContoller :type "/Game/AVRFramework/Blueprints/VR/MotionControllers/BP_BaseMotionController Object Reference"))
  (returns (Success :type Boolean))
  (set `self.Side` Side)
  (set `self.VRPawn` VRPawn)
  (set `self.ControllerComponent` MotionComponent)
  (set `self.BaseMotionController` MotionContoller)
  (return true))

(fn `SetVisibility`
  (params (Set :type Boolean)))

(fn `UpdateThumbstick`
  (params (ThumbstickUpAxis :type "Float (double-precision)") (ThumbstickRightAxis :type "Float (double-precision)"))
  (bind _active (`self.Active`))
  (bind _output_get (set `self.ThumbstickUpAxis` (`KismetMathLibrary.SelectFloat` ThumbstickUpAxis 0.0 _active)))
  (bind _output_get_2 (set `self.ThumbstickRightAxis` (`KismetMathLibrary.SelectFloat` ThumbstickRightAxis 0.0 _active)))
  (bind (_outrotation _nooffsetoutrotation) (`self.getRotationFromInput` _output_get _output_get_2))
  (set `self.ThumbstickRotation` _outrotation)
  (set `self.ThumbstickRotationNoOffset` _nooffsetoutrotation))

(fn `UserConstructionScript`)