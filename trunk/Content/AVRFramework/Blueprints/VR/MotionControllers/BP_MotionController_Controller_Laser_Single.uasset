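; Laser motion-controller Blueprint for the VR framework that favors a single laser on the right hand.
; It overrides ShouldLaserBeActive, allowing the right laser whenever the parent check passes.
; The left laser also requires the right controller to be holding an actor whose grab component has SnapAndReplaceControls set, found through the pawn's controller component map.
; BeginPlay, Tick and construction only call the parent.
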(event `self.ReceiveBeginPlay`
  (`parent.ReceiveBeginPlay`))

(event `self.ReceiveTick`
  (params (DeltaSeconds :type "Float (single-precision)"))
  (`parent.ReceiveTick` DeltaSeconds))

(fn `ShouldLaserBeActive`
  (returns (ShouldBeActive :type Boolean))
  (bind (_value _returnvalue) (`BlueprintMapLibrary.Map_Find` (`/Game/AVRFramework/Blueprints/VR/MotionControllers/BP_BaseMotionController.MCompMap` (`BlueprintMapLibrary.Map_Find` (`/Game/AVRFramework/Framework/BP_Pawn_VR.Controllers` (`self.VRPawn`)) "NewEnumerator1")) "NewEnumerator2"))
  (if (`parent.ShouldLaserBeActive`)
    (switch `/Game/AVRFramework/Enums/Enum_Side` (`self.Side`)
      (:`NewEnumerator0`
        (if _returnvalue
          (bind _grabbedactor (message `/Game/AVRFramework/Interface/Interface_GrabbingActor.getCurrentlyGrabbedActor` _value))
          (`/Engine/EditorBlueprintResources/StandardMacros.IsValid` _grabbedactor
            (:`Is Valid`
              (return (`/Game/AVRFramework/Blueprints/Components/Actor/Comp_Grab.SnapAndReplaceControls` (`self.GetComponentByClass` _grabbedactor "/Game/AVRFramework/Blueprints/Components/Actor/Comp_Grab.Comp_Grab_C"))))
            (:`Is Not Valid`
              (return false)))
          (else
            (return false))))
      (:`NewEnumerator1`
        (return true)))
    (else
      (return false))))

(fn `UserConstructionScript`
  (`parent.UserConstructionScript`))