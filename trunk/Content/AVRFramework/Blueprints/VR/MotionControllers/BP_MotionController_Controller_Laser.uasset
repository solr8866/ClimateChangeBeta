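; Motion controller variant with a laser pointer that switches off while the radial menu or teleporter is in use.
; Each Tick, after the parent's, it checks that two other components in MCompMap are inactive and sends the laser an interface active message, gated by a change-only macro.
; SetMeshVisibility shows or hides the laser and another mapped component together, mostly when a tool is taken.
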(event `self.ReceiveTick`
  (params (DeltaSeconds :type "Float (single-precision)"))
  (bind _shouldbeactive (`self.ShouldLaserBeActive`))
  (bind _value (`BlueprintMapLibrary.Map_Find` (`self.MCompMap`) "NewEnumerator2"))
  ;[1 1 1] Activate/Deactivate Laserpointer when opening Radial Menu or starting Teleporter
  (`parent.ReceiveTick` DeltaSeconds)
  (if (!= (`/Game/AVRFramework/Blueprints/VR/MotionComponents/BP_MComp.Active` (`BlueprintMapLibrary.Map_Find` (`self.MCompMap`) "NewEnumerator2")) _shouldbeactive)
    (if _shouldbeactive
      (message `/Game/AVRFramework/Interface/Interface_Active.Interface_SetActive` _value true)
      (else
        (message `/Game/AVRFramework/Interface/Interface_Active.Interface_SetActive` _value false)))))

(event `self.SetMeshVisibility`
  (params (Set :type Boolean))
  ;[1 1 1] Set Visiblity mostly when taking Tool
  (`/Game/AVRFramework/Blueprints/VR/MotionComponents/BP_MComp.SetVisibility` (`BlueprintMapLibrary.Map_Find` (`self.MCompMap`) "NewEnumerator2") Set)
  (`/Game/AVRFramework/Blueprints/VR/MotionComponents/BP_MComp.SetVisibility` (`BlueprintMapLibrary.Map_Find` (`self.MCompMap`) "NewEnumerator0") Set))

(fn `ShouldLaserBeActive`
  (returns (ShouldBeActive :type Boolean))
  (bind _mcompmap (`self.MCompMap`))
  (if (and (not (`/Game/AVRFramework/Blueprints/VR/MotionComponents/BP_MComp.Active` (`BlueprintMapLibrary.Map_Find` _mcompmap "NewEnumerator5"))) (not (`/Game/AVRFramework/Blueprints/VR/MotionComponents/BP_MComp.Active` (`BlueprintMapLibrary.Map_Find` _mcompmap "NewEnumerator7"))))
    (return true)
    (else
      (return false))))

(fn `UserConstructionScript`
  (`parent.UserConstructionScript`))