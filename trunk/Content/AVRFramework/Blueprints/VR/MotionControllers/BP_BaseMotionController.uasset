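; Base VR motion controller actor for one hand, hosting modular MComp child actors and routing controller input to them.
; It builds a map of MComps from its child actor components and resolves keys to functions through per-headset, per-side control mappings.
; A prioritised MComp receives raw keys and can block most mapped functions of other MComps.
; It also stores axis and touch values, highlights buttons, sets trim colour and scales with player size.
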(event `self.ReceiveTick`
  (params (DeltaSeconds :type "Float (single-precision)")))

(event `KeyInput`
  (params (Set :type Boolean) (Key :type "/Game/AVRFramework/Enums/Enum_MotionController_Buttons Enum" :default "NewEnumerator1"))
  (bind _prioritisedmcomp (`self.PrioritisedMComp`))
  ;[1 1 1] Assign Button Actions
  (bind _asbp_mcomp_controller (`self.GetControllerMComp`)
    (:`then`
      (`/Game/AVRFramework/Blueprints/VR/MotionComponents/BP_MComp_Controller.SetButtonHighlight` _asbp_mcomp_controller Key Set))
    (:`CastFailed`
      _))
  (`/Engine/EditorBlueprintResources/StandardMacros.IsValid` (`self.PrioritisedMComp`)
    (:`Is Valid`
      (`/Game/AVRFramework/Blueprints/VR/MotionComponents/BP_MComp.KeyInput` (`self.PrioritisedMComp`) Key Set))
    (:`Is Not Valid`
      _))
  (bind _infocontrols (`/Game/AVRFramework/Libraries/Lib_Core.getInfoControls` self))
  (bind _controllermeshoverride (`/Game/AVRFramework/Blueprints/Info/BP_Info_Controls.ControllerMeshOverride` _infocontrols))
  (bind (_value _returnvalue) (`BlueprintMapLibrary.Map_Find` (`/Game/AVRFramework/Blueprints/Info/BP_Info_Controls.FunctionMapping` _infocontrols) (select `bool` (`|EnumInequality` _controllermeshoverride "NewEnumerator0") :`false` (select `/Game/AVRFramework/Enums/Enum_HMD` (`self.HMD`) :`NewEnumerator0` "NewEnumerator1" :`NewEnumerator1` "NewEnumerator3" :`NewEnumerator2` "NewEnumerator0" :!type "/Game/AVRFramework/Enums/Enum_ControllerMeshes Enum") :`true` _controllermeshoverride)))
  (if _returnvalue
    (bind (_value_2 _returnvalue_2) (`BlueprintMapLibrary.Map_Find` (break `/Game/AVRFramework/Structs/Struct_SideToKeyMap` _value) (`self.Side`)))
    (if _returnvalue_2
      (bind (_value_3 _returnvalue_3) (`BlueprintMapLibrary.Map_Find` (break `/Game/AVRFramework/Structs/Struct_KeyToFunctionMap` _value_2) Key))
      (if _returnvalue_3
        (bind (_value_4 _returnvalue_4) (`BlueprintMapLibrary.Map_Find` (`self.AssignedFunctions`) _value_3))
        (if _returnvalue_4
          (bind (_value_5 _returnvalue_5) (`BlueprintMapLibrary.Map_Find` (`self.MCompMap`) _value_4))
          (if _returnvalue_5
            (if (or (`|EnumEquality` _value_3 "NewEnumerator2") (`|EnumEquality` _value_3 "NewEnumerator3"))
              (`/Game/AVRFramework/Blueprints/VR/MotionComponents/BP_MComp.FunctionInput` _value_5 _value_3 Set :!label _label)
              (else
                (`/Engine/EditorBlueprintResources/StandardMacros.IsValid` _prioritisedmcomp
                  (:`Is Valid`
                    (if (== _prioritisedmcomp _value_5)
                      (goto _label)))
                  (:`Is Not Valid`
                    (goto _label)))))))))))

(event `self.ReceiveBeginPlay`
  ;[1 1 1] Setup
  (`parent.ReceiveBeginPlay`)
  (set `MotionControllerComponent.MotionSource` (select `/Game/AVRFramework/Enums/Enum_Side` (`self.Side`) :`NewEnumerator0` "Left" :`NewEnumerator1` "Right" :!type "Name") (`self.MotionController`))
  (`self.UpdateMCompMap`))

(event `SetReplacedControls`
  (params (Set :type Boolean) (PriorityMComp :type "/Game/AVRFramework/Blueprints/VR/MotionComponents/BP_MComp Object Reference"))
  ;[1 1 1] Assign Button Actions
  (if Set
    (set `self.PrioritisedMComp` PriorityMComp)
    (else
      (set `self.PrioritisedMComp` null))))

(event `/Game/AVRFramework/Interface/Interface_Deleteable.Delete`
  (params (AnimToUse :type "/Game/AVRFramework/Enums/Enum_DeleteAppearAnim Enum" :default "NewEnumerator0"))
  ;[1 1 1] Delete Functionality
  (bind _result (`BlueprintSetLibrary.Set_ToArray` (`self.AttachedMComps`)))
  (for _array_element _result
    (`/Engine/EditorBlueprintResources/StandardMacros.IsValid` _array_element
      (:`Is Valid`
        (if (`KismetSystemLibrary.DoesImplementInterface` _array_element "/Game/AVRFramework/Interface/Interface_GrabbingActor.Interface_GrabbingActor_C")
          (message `/Game/AVRFramework/Interface/Interface_GrabbingActor.ReleaseActor` _array_element true)))))
  (`self.K2_DetachFromActor` "KeepRelative")
  (`self.SetActorHiddenInGame` true)
  (`self.K2_DestroyActor`))

(event `UpdateMCompMap`
  ;[1 1 1] Create MComp Map
  (`BlueprintMapLibrary.Map_Clear` (`self.MCompMap`))
  (for _array_element (`self.K2_GetComponentsByClass` "/Script/Engine.ChildActorComponent")
    (bind _asbp_mcomp (cast `/Game/AVRFramework/Blueprints/VR/MotionComponents/BP_MComp` (`ChildActorComponent.ChildActor` _array_element)))
    (`BlueprintMapLibrary.Map_Add` (`self.MCompMap`) (`/Game/AVRFramework/Blueprints/VR/MotionComponents/BP_MComp.MComp` _asbp_mcomp) _asbp_mcomp)))

(event `DesiredControllerColor`
  (params (DesiredColor :type "LinearColor Structure"))
  ;[1 1 1] AdjustVisuals
  (bind _asbp_mcomp_controller (`self.GetControllerMComp`)
    (:`then`
      (`/Game/AVRFramework/Blueprints/VR/MotionComponents/BP_MComp_Controller.SetTrimColor` _asbp_mcomp_controller DesiredColor))))

(event `SetMeshVisibility`
  (params (Set :type Boolean))
  ;[1 1 1] Set Visibility
)

(event `SetPLayerSize`
  (params (Size :type "Float (double-precision)"))
  ;[1 1 1] Adapt Controller Size if Player Size is changed
  (`SceneComponent.SetRelativeScale3D` (`self.MotionController`) (`KismetMathLibrary.Conv_DoubleToVector` Size)))

(fn `getAllAttachedActors`
  (returns (Actors :type "Set of Actor Object Reference"))
  (locals (Return :type "Set of Actor Object Reference"))
  (bind _return (`local.Return`))
  (bind _result (`BlueprintSetLibrary.Set_ToArray` (`self.AttachedMComps`)))
  (for _array_element _result
    (`/Engine/EditorBlueprintResources/StandardMacros.IsValid` _array_element
      (:`Is Valid`
        (bind _actors (`/Game/AVRFramework/Blueprints/VR/MotionComponents/BP_MComp.getAllAttachedActors` _array_element))
        (`BlueprintSetLibrary.Set_Union` _return _actors)
        (`BlueprintSetLibrary.Set_Add` _return _array_element))))
  (return (`local.Return`)))

(fn `GribAxis`
  (params (AxisValue :type "Float (double-precision)"))
  (set `self.Axis_Grib` AxisValue))

(fn `SetThumbstickRotation`
  (params (InRotation :type "Rotator Structure") (InRotationNoOffset :type "Rotator Structure") (InUpAxis :type "Float (double-precision)") (InRightAxis :type "Float (double-precision)"))
  (locals (LocalUpAxis :type "Float (double-precision)") (LocalRightAxis :type "Float (double-precision)") (LocalRotation :type "Rotator Structure") (LocalRotationNoOffset :type "Rotator Structure"))
  (set `local.LocalRotation` InRotation)
  (set `local.LocalRotationNoOffset` InRotationNoOffset)
  (set `local.LocalUpAxis` InUpAxis)
  (set `local.LocalRightAxis` InRightAxis)
  (set `self.ThumbstickRotation` (`local.LocalRotation`))
  (set `self.ThumbstickRotationNoOffset` (`local.LocalRotationNoOffset`))
  (set `self.Axis_Thumbstick_Up` (`local.LocalUpAxis`))
  (set `self.Aixs_Thumbstick_Right` (`local.LocalRightAxis`)))

(fn `ThumbCapTouch`
  (params (AxisValue :type "Float (double-precision)"))
  (set `self.Axis_Thumb_Touch` AxisValue))

(fn `TriggerAxis`
  (params (AxisValue :type "Float (double-precision)"))
  (set `self.Axis_Trigger` AxisValue))

(fn `TriggerCapTouch`
  (params (AxisValue :type "Float (double-precision)"))
  (set `self.Axis_Trigger_Touch` AxisValue))

(fn `UserConstructionScript`)