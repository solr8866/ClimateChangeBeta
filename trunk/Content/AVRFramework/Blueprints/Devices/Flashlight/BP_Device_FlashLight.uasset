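; BP_Device_FlashLight is a grabbable VR flashlight device in the AVR framework that the player switches on and off.
; Pressing the trigger on its grab component toggles the active state, which shows or hides the light and cone meshes, and plays a haptic pulse on the holding hand.
; Thumbstick input while grabbed adjusts the light intensity within clamped bounds.
; The construction script applies the default active state through the same interface.
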(event `self.ReceiveTick`
  (params (DeltaSeconds :type "Float (single-precision)")))

(event `self.Interface_SetConstructionActive`
  (params (Set :type Boolean))
  ;[1 1 1] Turn Flashlight On/Off
  (`self.Interface_SetActive` Set))

(event `self.Interface_SetActive`
  (params (Set :type Boolean))
  ;[1 1 1] Turn Flashlight On/Off
  (`SceneComponent.SetVisibility` (`self.MainLight`) Set false)
  (`SceneComponent.SetVisibility` (`self.SM_FlashLight_LightCone143`) Set false)
  (`SceneComponent.SetVisibility` (`self.SM_FlashLight_LightCone154`) Set false)
  (set `self.Active` Set))

(event `self.Interface_ToggleActive`
  ;[1 1 1] Turn Flashlight On/Off
  (`self.Interface_SetActive` (not (`self.Active`))))

(event `self.Comp_Grab.Thumbstick`
  (params (UpAxis :type "Float (single-precision)") (RightAxis :type "Float (single-precision)"))
  ;[1 1 1] Change Flashlight intensity with Thumbstick
  (if (or (> (`KismetMathLibrary.Abs` UpAxis) 0.0) (> (`KismetMathLibrary.Abs` RightAxis) 0.0))
    (`LightComponent.SetIntensity` (`self.MainLight`) (`KismetMathLibrary.FClamp` (+ (* UpAxis 30.0) (* RightAxis 30.0) (`LightComponentBase.Intensity` (`self.MainLight`))) 100.0 2000.0))))

(event `self.Comp_Grab.KeyInput`
  (params (Key :type "/Game/AVRFramework/Enums/Enum_MotionController_Buttons Enum" :default "NewEnumerator1") (Set :type Boolean))
  ;[1 1 1] Toggle Flashlight on Trigger Pressed
  (switch `/Game/AVRFramework/Enums/Enum_MotionController_Buttons` Key
    (:`NewEnumerator0`
      (if Set
        (`self.Interface_ToggleActive`)
        (`/Game/AVRFramework/Libraries/Lib_Core.SetHaptics` (`/Game/AVRFramework/Blueprints/Components/Actor/Comp_Grab.GrabbingMComp` (`self.Comp_Grab`)) "NewEnumerator1" (select `bool` (`self.Active`) :`false` "NewEnumerator2" :`true` "NewEnumerator1" :!type "/Game/AVRFramework/Enums/Enum_Haptic_Curves Enum") 0.1 1.0)))))

(fn `Interface_IsActive`
  (returns (IsActive :type Boolean))
  (return (`self.Active`)))

(fn `UserConstructionScript`
  (`parent.UserConstructionScript`)
  (`self.Interface_SetConstructionActive` (`self.Active`)))