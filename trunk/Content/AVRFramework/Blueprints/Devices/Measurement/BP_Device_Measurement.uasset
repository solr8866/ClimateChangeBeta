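; Grabbable VR measuring device that shows laser distance in cm or m and places linked measurement markers.
; Grabbing activates a laser child actor, and Tick traces forward, smoothing the endpoint and snapping it to highlighted existing markers.
; Trigger press starts a connection from a new or targeted marker, dragging the far end with haptics until release places or merges it.
; Face 02 sends a delete message to the targeted marker.
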(event `self.Comp_Grab.ActorPickedUp`
  (params (GrabbingPawn :type "/Game/AVRFramework/Framework/BP_Pawn_Base Object Reference") (GrabbingActor :type "Actor Object Reference") (GrabbingMotionController :type "/Game/AVRFramework/Blueprints/VR/MotionControllers/BP_BaseMotionController Object Reference") (GrabbingMComp :type "/Game/AVRFramework/Blueprints/VR/MotionComponents/BP_MComp Object Reference"))
  ;[1 1 1] Activate/Deactivate On Grab
  (`/Game/AVRFramework/Interface/Interface_Active.Interface_SetActive` true))

(event `self.Comp_Grab.ActorReleased`
  (bind _line (`self.Line`))
  ;[1 1 1] Activate/Deactivate On Grab
  (`/Game/AVRFramework/Interface/Interface_Active.Interface_SetActive` false)
  (`/Engine/EditorBlueprintResources/StandardMacros.IsValid` _line
    (:`Is Valid`
      (`ActorComponent.K2_DestroyComponent` _line))))

(event `Delete`
  (params (AnimToUse :type "/Game/AVRFramework/Enums/Enum_DeleteAppearAnim Enum" :default "NewEnumerator0"))
  ;[1 1 1] Handle Delete
)

(event `/Game/AVRFramework/Interface/Interface_Active.Interface_SetActive`
  (params (Set :type Boolean))
  (bind _lasercomponent (`self.LaserComponent`))
  ;[1 1 1] Set Active
  (bind _output_get (set `self.IsActive` Set))
  (if _output_get
    (`/Engine/EditorBlueprintResources/StandardMacros.IsValid` (`self.LaserComponent`)
      (:`Is Not Valid`
        (bind _returnvalue (`AddComponent|NODE_AddChildActorComponent-0`))
        (set `self.LaserComponent` _returnvalue)
        (bind _asbp_helper_laser (cast `/Game/AVRFramework/Blueprints/Helpers/BP_Helper_Laser` (`ChildActorComponent.ChildActor` _returnvalue)))
        (bind _output_get_2 (set `self.Laser` _asbp_helper_laser))
        (set `self.LastImpact` (+ (* (`self.GetActorForwardVector` _output_get_2) 20.0) (`SceneComponent.K2_GetComponentLocation` (`self.ArrowIndicator`))))))
    (else
      (`/Engine/EditorBlueprintResources/StandardMacros.IsValid` _lasercomponent
        (:`Is Valid`
          (`ActorComponent.K2_DestroyComponent` _lasercomponent)
          (set `self.LaserComponent` null)
          (set `self.Laser` null))))))

(event `self.Comp_Grab.KeyInput`
  (params (Key :type "/Game/AVRFramework/Enums/Enum_MotionController_Buttons Enum" :default "NewEnumerator1") (Set :type Boolean))
  (bind _measurementmarker (`self.MeasurementMarker`))
  (bind _measurementmarker_2 (`self.MeasurementMarker`))
  (bind _currentmeasurement (`self.CurrentMeasurement`))
  (bind _initialmeasurement (`self.InitialMeasurement`))
  (bind _currentconnection (`self.CurrentConnection`))
  ;[1 1 1] Place and Combine Measurement Marker
  (switch `/Game/AVRFramework/Enums/Enum_MotionController_Buttons` Key
    (:`NewEnumerator0`
      (if Set
        (`/Engine/EditorBlueprintResources/StandardMacros.IsValid` _measurementmarker
          (:`Is Valid`
            (set `self.InitialMeasurement` _measurementmarker))
          (:`Is Not Valid`
            (bind _returnvalue (`|SpawnActorFromClass` "/Game/AVRFramework/Blueprints/Helpers/BP_Helper_MeasurementMarker.BP_Helper_MeasurementMarker_C" (`KismetMathLibrary.MakeTransform` (`self.LastImpact`) (`self.LastRotation`)) "Undefined" "OverrideRootScale" null null))
            (set `self.InitialMeasurement` _returnvalue)))
        (bind _returnvalue_2 (`|SpawnActorFromClass` "/Game/AVRFramework/Blueprints/Helpers/BP_Helper_MeasurementMarker.BP_Helper_MeasurementMarker_C" (`KismetMathLibrary.MakeTransform` (`self.LastImpact`) (`self.LastRotation`)) "Undefined" "OverrideRootScale" null null))
        (set `self.CurrentMeasurement` _returnvalue_2)
        (bind _returnvalue_3 (`|SpawnActorFromClass` "/Game/AVRFramework/Blueprints/Helpers/BP_Helper_MeasurementConnection.BP_Helper_MeasurementConnection_C" (`self.GetTransform` _initialmeasurement) "Undefined" "OverrideRootScale" null _initialmeasurement (`self.CurrentMeasurement`) (`/Game/AVRFramework/Blueprints/Components/Actor/Comp_Grab.GrabbingPawn` (`self.Comp_Grab`)) null))
        (bind _output_get (set `self.CurrentConnection` _returnvalue_3))
        (`BlueprintSetLibrary.Set_Add` (`/Game/AVRFramework/Blueprints/Helpers/BP_Helper_MeasurementMarker.MeasurementConnections` (`self.InitialMeasurement`)) _output_get)
        (`BlueprintSetLibrary.Set_Add` (`/Game/AVRFramework/Blueprints/Helpers/BP_Helper_MeasurementMarker.MeasurementConnections` (`self.CurrentMeasurement`)) _output_get)
        (else
          (`/Engine/EditorBlueprintResources/StandardMacros.IsValid` _measurementmarker_2
            (:`Is Valid`
              (set `/Game/AVRFramework/Blueprints/Helpers/BP_Helper_MeasurementConnection.MeasurementMarkerB` _measurementmarker_2 _currentconnection)
              (`BlueprintSetLibrary.Set_Add` (`/Game/AVRFramework/Blueprints/Helpers/BP_Helper_MeasurementMarker.MeasurementConnections` _measurementmarker_2) _currentconnection)
              (`self.K2_DestroyActor` _currentmeasurement))
            (:`Is Not Valid`
              (set `/Game/AVRFramework/Blueprints/Helpers/BP_Helper_MeasurementMarker.Placed` true _currentmeasurement)))
          (set `self.CurrentMeasurement` null)
          (set `self.InitialMeasurement` null)
          (set `self.CurrentConnection` null))))
    (:`NewEnumerator4`
      (if Set
        (bind _measurementmarker_3 (`self.MeasurementMarker`)
          (:`then`
            (message `/Game/AVRFramework/Interface/Interface_Deleteable.Delete` _measurementmarker_3 "NewEnumerator1"))
          (:`else`))))))

(event `self.ReceiveTick`
  (params (DeltaSeconds :type "Float (single-precision)"))
  (bind _arrowindicator (`self.ArrowIndicator`))
  (bind _arrowindicator_2 (`self.ArrowIndicator`))
  (bind _returnvalue (`SceneComponent.K2_GetComponentLocation` _arrowindicator))
  (bind _returnvalue_2 (`SplineComponent.GetSplineLength` (`/Game/AVRFramework/Blueprints/Helpers/BP_Helper_Laser.HelperSpline` (`self.Laser`))))
  (bind _returnvalue_3 (>= _returnvalue_2 100.0))
  (bind _returnvalue_4 (select `bool` _returnvalue_3 :`false` 1 :`true` 2))
  ;[1 1 1] Check for Possible for Possible Location for Measurement Marker
  (`parent.ReceiveTick` DeltaSeconds)
  (set `self.DeltaSeconds` DeltaSeconds)
  (bind _isactive (`/Game/AVRFramework/Interface/Interface_Active.Interface_IsActive`))
  (if _isactive
    (bind _outhit (`KismetSystemLibrary.LineTraceSingle` _returnvalue (+ _returnvalue (* (`SceneComponent.GetForwardVector` _arrowindicator) 10000.0)) "TraceTypeQuery1" true (`|MakeArray` (`self.CurrentMeasurement`) :!type "Actor Object Reference")))
    (bind (_bblockinghit _binitialoverlap _time _distance _location _impactpoint _normal _impactnormal _physmat _hitactor) (`GameplayStatics.BreakHitResult` _outhit))
    (bind _asbp_helper_measurement_marker (cast `/Game/AVRFramework/Blueprints/Helpers/BP_Helper_MeasurementMarker` _hitactor)
      (:`then`
        (if (!= _asbp_helper_measurement_marker (`self.InitialMeasurement`))
          (bind _output_get (set `self.MeasurementMarker` _asbp_helper_measurement_marker))
          (`/Game/AVRFramework/Blueprints/Components/Actor/Comp_Highlight.SetHighlight` :`self` (`self.GetComponentByClass` _output_get "/Game/AVRFramework/Blueprints/Components/Actor/Comp_Highlight.Comp_Highlight_C") :`Set` true :`Color` "NewEnumerator5" :`ImpactLocation` _impactpoint :`MotionComponent` (`/Game/AVRFramework/Blueprints/Components/Actor/Comp_Grab.GrabbingMComp` (`self.Comp_Grab`)))
          (set `self.LastImpact` (`KismetMathLibrary.VInterpTo` (`self.LastImpact`) (`self.K2_GetActorLocation` _output_get) (`self.DeltaSeconds`) 20.0))
          (set `self.LastRotation` (`self.K2_GetActorRotation` _output_get))
          (`/Game/AVRFramework/Blueprints/Helpers/BP_Helper_Laser.SetLaserColor` (`self.Laser`) 100.0 (`self.DeltaSeconds`) true (struct :`R` 0.65625 :`G` 0.026995 :`A` 1.0) 1.0 (1.0 1.0) (1.0 1.0))
          (else
            (set `self.MeasurementMarker` null :!label _label)
            (set `self.LastImpact` (`KismetMathLibrary.VInterpTo` (`self.LastImpact`) _impactpoint (`self.DeltaSeconds`) 20.0))
            (set `self.LastRotation` (`KismetMathLibrary.MakeRotFromZ` _impactnormal))
            (`/Game/AVRFramework/Blueprints/Helpers/BP_Helper_Laser.SetLaserColor` (`self.Laser`) 100.0 (`self.DeltaSeconds`) true (struct :`R` 1.0 :`G` 0.272749 :`A` 1.0) 1.0 (1.2 1.2) (1.2 1.2)))))
      (:`CastFailed`
        (goto _label)))
    (`/Game/AVRFramework/Blueprints/Helpers/BP_Helper_Laser.UpdateLaser` (`self.Laser`) (`SceneComponent.K2_GetComponentLocation` _arrowindicator_2) (`self.LastImpact`) (`SceneComponent.GetForwardVector` _arrowindicator_2))
    (`TextRenderComponent.K2_SetText` (`self.Number`) (`KismetTextLibrary.Conv_DoubleToText` (select `bool` _returnvalue_3 :`false` _returnvalue_2 :`true` (/ _returnvalue_2 100.0)) "HalfToEven" false true 1 324 _returnvalue_4 _returnvalue_4))
    (`TextRenderComponent.K2_SetText` (`self.TextRender1`) (select `bool` _returnvalue_3 :`false` "cm" :`true` "m"))
    (bind _currentmeasurement (`self.CurrentMeasurement`)
      (:`then`
        (`self.K2_SetActorLocationAndRotation` _currentmeasurement (`self.LastImpact`) (`KismetMathLibrary.RInterpTo` (`self.K2_GetActorRotation` _currentmeasurement) (`self.LastRotation`) (`self.DeltaSeconds`) 20.0) false false)
        (`/Game/AVRFramework/Libraries/Lib_Core.SetHaptics` (`/Game/AVRFramework/Blueprints/Components/Actor/Comp_Grab.GrabbingMComp` (`self.Comp_Grab`)) "NewEnumerator1" "NewEnumerator4" 0.0 0.1))
      (:`else`))))

(fn `Interface_IsActive`
  (returns (IsActive :type Boolean))
  (return (`self.IsActive`)))

(fn `UserConstructionScript`
  (`parent.UserConstructionScript`))