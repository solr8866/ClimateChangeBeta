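; Grabbable VR pen device that draws 3D strokes in the air.
; Each trigger press spawns a BP_Helper_Splinedrawing, which Tick feeds with tip position, material and thumbstick-adjusted width while held, with haptics scaled to width.
; Face 02 toggles a BP_ColorPallet facing the user, removed on release; ChangeDrawingMaterial sets the stroke material and tints the pen to match.
; A line-trace widget selection for the palette is unfinished and disconnected.
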(event `/Game/AVRFramework/Interface/Interface_Deleteable.Delete`
  (params (AnimToUse :type "/Game/AVRFramework/Enums/Enum_DeleteAppearAnim Enum" :default "NewEnumerator0"))
  ;[1 1 1] Delete
  (`/Game/AVRFramework/Libraries/MLib_Actor_Macros.DeleteActorsAndWait` (`|MakeArray` (`self.ColorPallet`) :!type "Actor Object Reference")
    (:`AllGone`
      (`self.K2_DestroyActor`))))

(event `self.ReceiveBeginPlay`)

(event `self.Comp_Grab.KeyInput`
  (params (Key :type "/Game/AVRFramework/Enums/Enum_MotionController_Buttons Enum" :default "NewEnumerator1") (Set :type Boolean))
  (bind _arrow (`self.Arrow`))
  (bind _returnvalue (+ (`self.K2_GetActorLocation`) (0.0 0.0 20.0)))
  ;[1 1 1] On Triggerpressed create SplineDrawing Actor
  (switch `/Game/AVRFramework/Enums/Enum_MotionController_Buttons` Key
    (:`NewEnumerator0`
      (if Set
        (bind _returnvalue_2 (`|SpawnActorFromClass` "/Game/AVRFramework/Blueprints/Helpers/BP_Helper_Splinedrawing.BP_Helper_Splinedrawing_C" (`KismetMathLibrary.MakeTransform` (`SceneComponent.K2_GetComponentLocation` _arrow) (`SceneComponent.K2_GetComponentRotation` _arrow)) "Undefined" "OverrideRootScale" null null))
        (set `self.SplineDrawing` _returnvalue_2)
        (set `self.IsDrawing` true)
        (else
          (set `self.IsDrawing` false))))
    (:`NewEnumerator4`
      (if Set
        (`/Engine/EditorBlueprintResources/StandardMacros.IsValid` (`self.ColorPallet`)
          (:`Is Valid`
            (message `/Game/AVRFramework/Interface/Interface_Deleteable.Delete` (`self.ColorPallet`) "NewEnumerator1")
            (set `self.ColorPallet` null))
          (:`Is Not Valid`
            (bind _grabbingpawn (`/Game/AVRFramework/Blueprints/Components/Actor/Comp_Grab.CurrentlyGrabbedBy` (`self.Comp_Grab`)))
            (bind _returnvalue_3 (`|SpawnActorFromClass` "/Game/AVRFramework/Blueprints/UI/Utils/BP_ColorPallet.BP_ColorPallet_C" (`KismetMathLibrary.MakeTransform` _returnvalue (`KismetMathLibrary.FindLookAtRotation` _returnvalue (`SceneComponent.K2_GetComponentLocation` (`/Game/AVRFramework/Framework/BP_Pawn_Base.GetCameraComponent` _grabbingpawn)))) "Undefined" "OverrideRootScale" null self null))
            (set `self.ColorPallet` _returnvalue_3)))))))

(event `ChangeDrawingMaterial`
  (params (SplineMaterial :type "MaterialInterface Object Reference"))
  ;[1 1 1] Handle Change Drawing Color
  (bind _output_get (set `self.SplineMaterial` SplineMaterial))
  (bind _returnvalue (`KismetMaterialLibrary.CreateDynamicMaterialInstance` _output_get _output_get))
  (bind _output_get_2 (set `self.DynamicSplineMaterial` _returnvalue))
  (bind _returnvalue_2 (`MaterialInstanceDynamic.K2_GetVectorParameterValue` _output_get_2 "Color"))
  (bind _returnvalue_3 (`KismetMathLibrary.Conv_LinearColorToVector` _returnvalue_2))
  (`MeshComponent.SetVectorParameterValueOnMaterials` (`self.PenMesh`) "Color" _returnvalue_3)
  (`MeshComponent.SetVectorParameterValueOnMaterials` (`self.Tip`) "Color" (/ _returnvalue_3 3.0)))

(event `self.Comp_Grab.Thumbstick`
  (params (UpAxis :type "Float (single-precision)") (RightAxis :type "Float (single-precision)"))
  ;[1 1 1] Change Drawing Size based on Thumbstick
  (set `self.Scale` (`KismetMathLibrary.FClamp` (+ (`self.Scale`) (* RightAxis 0.2)) 0.2 3.0)))

(event `self.ReceiveTick`
  (params (DeltaSeconds :type "Float (single-precision)"))
  ;[1 1 1] Event Tick
  (`parent.ReceiveTick` DeltaSeconds)
  (set `self.DeltaSeconds` DeltaSeconds)
  ;[1 1 1] Create New Drawing Spline Points
  (if (`self.IsDrawing`)
    (`/Game/AVRFramework/Blueprints/Helpers/BP_Helper_Splinedrawing.NewPenLocation` (`self.SplineDrawing`) (`SceneComponent.K2_GetComponentLocation` (`self.Arrow`)) (`self.SplineMaterial`) (`self.Scale`))
    (`/Game/AVRFramework/Libraries/Lib_Core.SetHaptics` (`/Game/AVRFramework/Blueprints/Components/Actor/Comp_Grab.GrabbingMComp` (`self.Comp_Grab`)) "NewEnumerator1" "NewEnumerator4" 0.0 (`KismetMathLibrary.MapRangeUnclamped` (`self.Scale`) 0.2 3.0 0.1 0.3))))

(event `self.Comp_Grab.ActorReleased`
  ;[1 1 1] Destroy Color Pallet if valid
  (bind _colorpallet (`self.ColorPallet`)
    (:`then`
      (`/Game/AVRFramework/Blueprints/UI/Utils/BP_ColorPallet.Delete` _colorpallet "NewEnumerator1"))
    (:`else`)))

(fn `UserConstructionScript`
  (`parent.UserConstructionScript`)
  (`self.ChangeDrawingMaterial` (`self.SplineMaterial`)))