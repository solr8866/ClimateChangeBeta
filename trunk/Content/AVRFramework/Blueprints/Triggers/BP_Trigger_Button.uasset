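; VR push-button trigger that fires set/unset section events, working as a toggle or hold-to-activate button.
; While a component overlaps it (optionally only BP_MComp), Tick sinks the button by the computed push distance with proportional haptics.
; Full depth or selection triggers sound, haptic pulse, pressed callback and a timeline-driven red/green material change.
; Ending overlap animates the button back and releases it in hold mode.
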(event `self.ReceiveBeginPlay`
  ;[1 1 1] Setup
  (set `self.OriginalButtonLocation` (`SceneComponent.RelativeLocation` (`self.Button`)))
  (bind _returnvalue (`PrimitiveComponent.CreateDynamicMaterialInstance` (`self.Button`) 0 null "None"))
  (set `self.ButtonMaterial` _returnvalue))

(event `/Game/AVRFramework/Interface/Interface_ListenToTrigger.Interface_TriggerSingleToggle`
  (params (Source :type "Actor Object Reference"))
  (bind _interactingcomponent (`self.InteractingComponent`))
  ;[1 1 1] SimulateButtonPhysics
  (`GameplayStatics.PlaySoundAtLocation` "/Game/AVRFramework/Sound/Cues/Buttons/Cue_Button_Pressed.Cue_Button_Pressed" (`SceneComponent.K2_GetComponentLocation` (`self.Button`)) (struct) 1.0 1.0 0.0 null null null :!label _label)
  (`self.Pressed`)
  (`/Engine/EditorBlueprintResources/StandardMacros.IsValid` _interactingcomponent
    (:`Is Valid`
      (bind _asbp_mcomp (cast `/Game/AVRFramework/Blueprints/VR/MotionComponents/BP_MComp` (`ActorComponent.GetOwner` _interactingcomponent))
        (:`then`
          (`/Game/AVRFramework/Libraries/Lib_Core.SetHaptics` _asbp_mcomp "NewEnumerator3" "NewEnumerator4" 0.2 1.0))
        (:`CastFailed`
          _)))
    (:`Is Not Valid`
      _))
  (if (`self.HoldingButton`)
    (`self.SetButtonState` true)
    (`self.EventTriggerSingle` (`self.SetSection`))
    (else
      (`self.SetButtonState` (not (`self.Set`)))
      (`self.EventTriggerSingle` (select `bool` (`self.Set`) :`false` (`self.UnsetSection`) :`true` (`self.SetSection`))))))

(event `self.ReceiveTick`
  (params (DeltaSeconds :type "Float (single-precision)"))
  (bind _button (`self.Button`))
  (bind (_returnvalue_x _returnvalue_y _returnvalue_z) (`KismetMathLibrary.BreakVector` (- (`KismetMathLibrary.InverseTransformDirection` (`SceneComponent.K2_GetComponentToWorld` _button) (`self.TrackingLocation`)) (`KismetMathLibrary.InverseTransformDirection` (`SceneComponent.K2_GetComponentToWorld` _button) (`SceneComponent.K2_GetComponentLocation` (`self.InteractingComponent`))))))
  ;[1 1 1] SimulateButtonPhysics
  (`/Engine/EditorBlueprintResources/StandardMacros.IsValid` (`self.InteractingComponent`)
    (:`Is Valid`
      (set `self.CurrentButtonDistance` (`KismetMathLibrary.FClamp` _returnvalue_z 0.0 (`self.RequiredButtonDistance`)))
      (`SceneComponent.K2_SetRelativeLocation` (`self.Button`) (- (`self.OriginalButtonLocation`) (`KismetMathLibrary.MakeVector` 0.0 0.0 (`self.CurrentButtonDistance`))) false false)
      (bind _asbp_mcomp (cast `/Game/AVRFramework/Blueprints/VR/MotionComponents/BP_MComp` (`ActorComponent.GetOwner` (`self.InteractingComponent`)))
        (:`then`
          (`/Game/AVRFramework/Libraries/Lib_Core.SetHaptics` _asbp_mcomp "NewEnumerator3" "NewEnumerator4" 0.0 (/ (`self.CurrentButtonDistance`) (`self.RequiredButtonDistance`))))
        (:`CastFailed`
          _))
      (if (>= (`self.CurrentButtonDistance`) (`self.RequiredButtonDistance`))
        (`/Engine/EditorBlueprintResources/StandardMacros.DoOnce` false :!label _label_2
          (:`Completed`
            (goto _label)))
        (else
          (goto _label_2 :!via `Reset`))))))

(event `/Game/AVRFramework/Interface/Interface_Selectable.SelectPressed`
  (params (Pawn :type "/Game/AVRFramework/Framework/BP_Pawn_Base Object Reference") (BaseMotionController :type "/Game/AVRFramework/Blueprints/VR/MotionControllers/BP_BaseMotionController Object Reference") (MotionController :type "MotionControllerComponent Object Reference") (MComp :type "/Game/AVRFramework/Blueprints/VR/MotionComponents/BP_MComp Object Reference") (ImpactLocation :type "Vector Structure") (ImpactComponent :type "ActorComponent Object Reference"))
  ;[1 1 1] SimulateButtonPhysics
  (goto _label))

(event `SetButtonState`
  (params (Set :type Boolean))
  ;[1 1 1] ButtonColorChange
  (set `self.Set` Set)
  (if Set
    (bind (_direction _procent) (`Timeline|ButtonTimeline` :!label _label_3)
      (:`Update`
        (`MaterialInstanceDynamic.SetScalarParameterValue` (`self.ButtonMaterial`) "FresnelExponent" (`KismetMathLibrary.Lerp` 0.3 2.0 _procent))
        (`MaterialInstanceDynamic.SetVectorParameterValue` (`self.ButtonMaterial`) "Color" (`KismetMathLibrary.LinearColorLerp` (struct :`R` 1.0 :`A` 1.0) (struct :`G` 1.0 :`A` 1.0) _procent))))
    (else
      (goto _label_3 :!via `Reverse`))))

(event `PlayReset`
  (params (Stop :type Boolean))
  ;[1 1 1] Reset Timeline
  (if Stop
    (bind (_direction _procent) (`Timeline|Reset` :!via `Stop` :!label _label_4)
      (:`Update`
        (`SceneComponent.K2_SetRelativeLocation` (`self.Button`) (`KismetMathLibrary.VLerp` (`self.TemporaryLocation`) (`self.OriginalButtonLocation`) _procent) false false)))
    (else
      (set `self.TemporaryLocation` (`SceneComponent.RelativeLocation` (`self.Button`)))
      (goto _label_4 :!via `PlayFromStart`))))

(event `self.Button.OnComponentBeginOverlap`
  (params (OverlappedComponent :type "PrimitiveComponent Object Reference") (OtherActor :type "Actor Object Reference") (OtherComp :type "PrimitiveComponent Object Reference") (OtherBodyIndex :type Integer) (bFromSweep :type Boolean) (SweepResult :type "HitResult Structure (by ref)"))
  ;[1 1 1] Overlap Events
  (`self.InteractingComponent`
    (:`then`)
    (:`else`
      (if (`self.OnlyTriggerByMComp`)
        (cast `/Game/AVRFramework/Blueprints/VR/MotionComponents/BP_MComp` OtherActor))
      (bind _output_get (set `self.InteractingComponent` OtherComp))
      (set `self.TrackingLocation` (`SceneComponent.K2_GetComponentLocation` _output_get))
      (`self.PlayReset` true))))

(event `self.Button.OnComponentEndOverlap`
  (params (OverlappedComponent :type "PrimitiveComponent Object Reference") (OtherActor :type "Actor Object Reference") (OtherComp :type "PrimitiveComponent Object Reference") (OtherBodyIndex :type Integer))
  ;[1 1 1] Overlap Events
  (if (== OtherComp (`self.InteractingComponent`))
    (set `self.InteractingComponent` null)
    (`self.PlayReset` false)
    (if (and (`self.HoldingButton`) (`self.Set`))
      (`self.SetButtonState` false)
      (`self.Released`)
      (`self.EventTriggerSingle` (`self.UnsetSection`)))))

(fn `CanBeSelected`
  (returns (IsSelectable :type Boolean))
  (return true))

(fn `UserConstructionScript`)