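; Base VR drag trigger that slides a mesh along a one-dimensional position range defined by Sections, with GetTransformFromPosition as an apparent override point.
; While dragged, Tick eases toward the dragging helper, probing a small step along the path and using angle and distance to find the target.
; Release coasts, snaps to the nearest segment or resets, via timelines.
; Position updates can fire segment and continuous trigger events plus movement-scaled haptics.
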(event `/Game/AVRFramework/Interface/Interface_Draggable.DragPressed`
  (params (VRPawn :type "/Game/AVRFramework/Framework/BP_Pawn_Base Object Reference") (GrabbingActor :type "Actor Object Reference") (MotionController :type "/Game/AVRFramework/Blueprints/VR/MotionControllers/BP_BaseMotionController Object Reference") (MComp :type "/Game/AVRFramework/Blueprints/VR/MotionComponents/BP_MComp Object Reference") (DraggingHelper :type "/Game/AVRFramework/Blueprints/Helpers/BP_Helper_Drag Object Reference"))
  (bind (_minvalue _maxvalue) (`self.SectionExtremes`))
  ;[1 1 1] Handle Drag
  (set `self.DraggingVRPawn` VRPawn)
  (set `self.DraggingMotionController` MotionController)
  (set `self.DraggingMComp` MComp)
  (set `self.DraggingHelper` DraggingHelper)
  ;[1 1 1] Set Offset
  (`|ExecutionSequence`
    (:`then_0`
      ;[1 1 1] After Release (Snap or Free Movement)
      (switch `/Game/AVRFramework/Enums/Enum_Drag_Type` (`self.DragType`)
        (:`NewEnumerator0`
          (bind (_direction _procent) (`Timeline|StopTimeline` :!via `Stop` :!label _label)
            (:`Update`
              (`self.SetNewPosition` (`KismetMathLibrary.FClamp` (+ (`self.CurrentPosition`) (* _procent (stale `/Game/AVRFramework/Interface/Interface_Draggable.DragRelease` _out) (`GameplayStatics.GetWorldDeltaSeconds`))) _minvalue _maxvalue)))))
        (:`NewEnumerator1`
          (bind (_direction_2 _procent_2) (`Timeline|SnappingTimeline` :!via `Stop` :!label _label_2)
            (:`Update`
              (`self.SetNewPosition` (`KismetMathLibrary.Lerp` (stale `/Game/AVRFramework/Interface/Interface_Draggable.DragRelease` _out_2) (select `/Game/AVRFramework/Enums/Enum_Drag_Type` (`self.DragType`) :`NewEnumerator1` (`self.ClosestSegment`) :`NewEnumerator2` (`self.OriginalLocation`)) _procent_2)))))
        (:`NewEnumerator2`
          (goto _label_2 :!via `Stop`))))
    (:`then_1`
      (bind (_haspoint _location) (`/Game/AVRFramework/Interface/Interface_Draggable.getDragDesiredAttachpoint`))
      (`SceneComponent.K2_SetWorldLocation` (`self.Offset`) (select `bool` _haspoint :`false` (`self.K2_GetActorLocation` (`self.DraggingHelper`)) :`true` _location) false false))))

(event `/Game/AVRFramework/Interface/Interface_Draggable.DragRelease`
  ;[1 1 1] Handle Drag
  (set `self.DraggingVRPawn` null)
  (set `self.DraggingMotionController` null)
  (set `self.DraggingMComp` null)
  (set `self.DraggingHelper` null)
  ;[1 1 1] After Release (Snap or Free Movement)
  (switch `/Game/AVRFramework/Enums/Enum_Drag_Type` (`self.DragType`)
    (:`NewEnumerator0`
      (bind _out (`/Game/AVRFramework/Libraries/FLib_Utility.SaveFloat` (/ (`self.MovementDelta`) (`GameplayStatics.GetWorldDeltaSeconds`))))
      (goto _label :!via `PlayFromStart`))
    (:`NewEnumerator1`
      _)
    (:`NewEnumerator2`
      _))
  (`TimelineComponent.SetPlayRate` (`self.SnappingTimeline`) (`KismetMathLibrary.MapRangeClamped` (`KismetMathLibrary.Abs` (- (`self.CurrentPosition`) (select `/Game/AVRFramework/Enums/Enum_Drag_Type` (`self.DragType`) :`NewEnumerator1` (`self.ClosestSegment`) :`NewEnumerator2` (`self.OriginalLocation`)))) 0.0 300.0 5.0 0.7))
  (bind _out_2 (`/Game/AVRFramework/Libraries/FLib_Utility.SaveFloat` (`self.CurrentPosition`)))
  (goto _label_2 :!via `PlayFromStart`))

(event `self.ReceiveBeginPlay`
  (`parent.ReceiveBeginPlay`)
  (set `self.OriginalLocation` (`self.CurrentPosition`))
  (set `self.LastSegment` (`self.ClosestSegment`)))

(event `SetNewPosition`
  (params (NewPosition :type "Float (double-precision)") (CallTrigger :type Boolean :default true))
  (bind (_minvalue _maxvalue) (`self.SectionExtremes`))
  (bind _closestpoint (`self.ClosestSegment`))
  (bind _value (`BlueprintMapLibrary.Map_Find` (`self.Sections`) _closestpoint))
  ;[1 1 1] Set New relative Position
  (set `self.MovementDelta` (- NewPosition (`self.CurrentPosition`)))
  (bind _output_get (set `self.CurrentPosition` NewPosition))
  (`SceneComponent.K2_SetRelativeTransform` (`self.MeshHandle`) (`self.getTransformFromPosition` _output_get) false false)
  (`SceneComponent.K2_SetRelativeTransform` (`self.OffsetHandle`) (`self.getTransformFromPosition` _output_get) false false)
  (if CallTrigger
    (if (not (!= (`self.LastSegment`) _closestpoint))
      (`self.EventTriggerSingle` _value)
      (set `self.LastSegment` _closestpoint))
    (`self.EventTriggerConstant` _value (`self.CurrentPosition`) (`KismetMathLibrary.NormalizeToRange` (`self.CurrentPosition`) _minvalue _maxvalue) (`self.MovementDelta`))
    (`/Game/AVRFramework/Libraries/Lib_Core.SetHaptics` (`self.DraggingMComp`) "NewEnumerator3" "NewEnumerator4" 0.0 (`self.MovementDelta`))))

(event `self.ReceiveTick`
  (params (DeltaSeconds :type "Float (single-precision)"))
  ;[1 1 1] Follow Dragging Helper
  (`self.DraggingHelper`
    (:`then`
      (`self.SetNewPosition` (`KismetMathLibrary.FInterpTo` (`self.CurrentPosition`) (`self.SearchForBestPointToOffset`) (`GameplayStatics.GetWorldDeltaSeconds`) (`self.FollowSpeed`))))
    (:`else`)))

(fn `CanBeDragged`
  (params (HitComponent :type "ActorComponent Object Reference"))
  (returns (IsDraggable :type Boolean))
  (return true))

(fn `ClosestSegment`
  (returns (ClosestPoint :type "Float (double-precision)"))
  (locals (Reference :type "Float (double-precision)" :default 100000.0))
  (bind _keys (`BlueprintMapLibrary.Map_Keys` (`self.Sections`)))
  (for _array_element _keys
    (if (< (`KismetMathLibrary.Abs` (- _array_element (`self.CurrentPosition`))) (`KismetMathLibrary.Abs` (- (`local.Reference`) (`self.CurrentPosition`))))
      (set `local.Reference` _array_element)))
  (return (`local.Reference`)))

(fn `CurrentlyDraggedBy`
  (returns (VRPawn :type "/Game/AVRFramework/Framework/BP_Pawn_Base Object Reference") (BsseMotionController :type "/Game/AVRFramework/Blueprints/VR/MotionControllers/BP_BaseMotionController Object Reference") (MComp :type "/Game/AVRFramework/Blueprints/VR/MotionComponents/BP_MComp Object Reference"))
  (return (`self.DraggingVRPawn`) (`self.DraggingMotionController`) (`self.DraggingMComp`)))

(fn `getDragDesiredAttachpoint`
  (returns (HasPoint :type Boolean) (Location :type "Vector Structure"))
  (return false (0.0 0.0 0.0)))

(fn `getTransformFromPosition`
  (params (Position :type "Float (double-precision)"))
  (returns (Transform :type "Transform Structure"))
  (return (`SceneComponent.GetRelativeTransform` (`self.MeshHandle`))))

(fn `SearchForBestPointToOffset`
  (returns (ClosestPosition :type "Float (double-precision)"))
  (locals (CurrentClosestDistance :type "Float (double-precision)" :default 0.0) (Counter :type "Float (double-precision)") (Direction :type Boolean))
  (bind (_minvalue _maxvalue) (`self.SectionExtremes`))
  (bind (_minvalue_2 _maxvalue_2) (`self.SectionExtremes`))
  (bind _returnvalue_location (`KismetMathLibrary.BreakTransform` (`SceneComponent.K2_GetComponentToWorld` (`self.Offset`))))
  (bind _returnvalue (`SceneComponent.K2_GetComponentLocation` (`self.Offset`)))
  (bind _returnvalue_2 (+ (`self.CurrentPosition`) 0.1))
  (bind _returnvalue_3 (`KismetMathLibrary.FClamp` _returnvalue_2 _minvalue_2 _maxvalue_2))
  (`SceneComponent.K2_SetRelativeTransform` (`self.OffsetHandle`) (`self.getTransformFromPosition` (`self.CurrentPosition`)) false false)
  (bind _out (`/Game/AVRFramework/Libraries/FLib_Utility.SaveVector` (- (`self.K2_GetActorLocation` (`self.DraggingHelper`)) _returnvalue_location)))
  (bind _out_2 (`/Game/AVRFramework/Libraries/FLib_Utility.SaveVector` (`SceneComponent.K2_GetComponentLocation` (`self.Offset`))))
  (bind _out_3 (`/Game/AVRFramework/Libraries/FLib_Utility.SaveBool` (== _returnvalue_2 _returnvalue_3)))
  (`SceneComponent.K2_SetRelativeTransform` (`self.OffsetHandle`) (`self.getTransformFromPosition` (select `bool` _out_3 :`false` (- (`self.CurrentPosition`) 0.1) :`true` _returnvalue_3)) false false)
  (bind _angle (`/Game/AVRFramework/Libraries/FLib_Utility.CalculateAngleFrom2Vectors` _out (select `bool` _out_3 :`false` (- _out_2 _returnvalue) :`true` (- _returnvalue _out_2))))
  (bind (_negative _value) (`/Game/AVRFramework/Libraries/MLib_Object_Macros.ValueAndNegative` (`KismetMathLibrary.VSize` _out)))
  (return (`KismetMathLibrary.FClamp` (+ (`self.CurrentPosition`) (select `bool` (< _angle 90.0) :`false` (`KismetMathLibrary.MapRangeClamped` _angle 180.0 90.0 _negative) :`true` (`KismetMathLibrary.MapRangeClamped` _angle 0.0 90.0 _value))) _minvalue _maxvalue)))

(fn `SectionExtremes`
  (returns (MinValue :type "Float (double-precision)") (MaxValue :type "Float (double-precision)"))
  (bind _keys (`BlueprintMapLibrary.Map_Keys` (`self.Sections`)))
  (return (`.MinValue` (`KismetMathLibrary.MinOfFloatArray` _keys)) (`.MaxValue` (`KismetMathLibrary.MaxOfFloatArray` _keys))))

(fn `UserConstructionScript`
  (bind (_minvalue _maxvalue) (`self.SectionExtremes`))
  (`self.SetNewPosition` (`KismetMathLibrary.FClamp` (`self.CurrentPosition`) _minvalue _maxvalue)))