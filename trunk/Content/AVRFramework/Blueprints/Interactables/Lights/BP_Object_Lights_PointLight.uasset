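; Point light interactable in the AVR framework whose root mesh material mirrors the light's brightness and color.
; On a light value update it runs the parent logic, then sets the material's Brightness parameter from the percentage, lerped up to a fixed maximum.
; A color update event copies the PointLight component's color into the material's Color parameter.
; Each update creates a dynamic material instance on the root's first slot.
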(event `self.Interface_UpdateLightValue`
  (params (Procent :type "Float (single-precision)"))
  (`parent.Interface_UpdateLightValue` Procent)
  (bind _returnvalue (`PrimitiveComponent.CreateDynamicMaterialInstance` (`self.Root`) 0 null "None"))
  (`MaterialInstanceDynamic.SetScalarParameterValue` _returnvalue "Brightness" (`KismetMathLibrary.Lerp` 0.0 20.0 Procent)))

(event `UpdateLightColor`
  (bind _returnvalue (`PrimitiveComponent.CreateDynamicMaterialInstance` (`self.Root`) 0 null "None"))
  (`MaterialInstanceDynamic.SetVectorParameterValue` _returnvalue "Color" (`LightComponentBase.GetLightColor` (`self.PointLight`))))

(fn `UserConstructionScript`
  (`parent.UserConstructionScript`))