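; Interactable light object in the AVR framework that switches and fades all of its light components on or off.
; Set and toggle calls play or reverse a timeline whose progress scales every light's intensity between zero and a configured value.
; Single, toggle and constant trigger interface events drive it, with constant triggers setting brightness directly by percentage.
; The construction script moves the timeline to match the initial on/off state.
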(event `self.Interface_SetConstructionLight`
  (params (Set :type Boolean))
  ;[1 1 1] Handle Turn On/Off Lights
  (`/Game/AVRFramework/Libraries/MLib_Object_Macros.ManipulateTimeline` (`self.LightTimeline`) Set))

(event `self.Interface_SetLight`
  (params (Set :type Boolean))
  ;[1 1 1] Handle Turn On/Off Lights
  (bind _output_get (set `self.LightOn` Set))
  (if _output_get
    (bind (_direction _procent) (`Timeline|LightTimeline` :!label _label)
      (:`Update`
        (`self.Interface_UpdateLightValue` _procent)))
    (else
      (goto _label :!via `Reverse`))))

(event `self.Interface_UpdateLightValue`
  (params (Procent :type "Float (single-precision)"))
  ;[1 1 1] Handle Turn On/Off Lights
  (for _array_element (`self.K2_GetComponentsByClass` "/Script/Engine.LightComponent")
    (`LightComponent.SetIntensity` _array_element (`KismetMathLibrary.Lerp` 0.0 (`self.LightValue`) Procent))))

(event `self.Interface_ToggleLight`
  ;[1 1 1] Handle Turn On/Off Lights
  (bind _islight (`self.Interface_IsLight`))
  (`self.Interface_SetLight` (not _islight)))

(event `/Game/AVRFramework/Interface/Interface_ListenToTrigger.Interface_TriggerSingle`
  (params (Section :type "/Game/AVRFramework/Structs/Struct_Section Structure") (Source :type "Actor Object Reference"))
  ;[1 1 1] Trigger Responses
  (`self.Interface_SetLight` Section_Set_10_F815F62F4975A2161C6C1E96D17A49FF))

(event `/Game/AVRFramework/Interface/Interface_ListenToTrigger.Interface_TriggerConstant`
  (params (Name :type Name) (Distance :type "Float (single-precision)") (Procent :type "Float (single-precision)") (Set :type Boolean) (Velocity :type "Float (single-precision)") (Source :type "Actor Object Reference"))
  ;[1 1 1] Trigger Responses
  (`self.Interface_UpdateLightValue` Procent))

(event `/Game/AVRFramework/Interface/Interface_ListenToTrigger.Interface_TriggerSingleToggle`
  (params (Source :type "Actor Object Reference"))
  ;[1 1 1] Trigger Responses
  (`self.Interface_ToggleLight`))

(fn `Interface_IsLight`
  (returns (IsLight :type Boolean))
  (return (`self.LightOn`)))

(fn `UserConstructionScript`
  (`parent.UserConstructionScript`)
  (`self.Interface_SetConstructionLight` (`self.LightOn`)))