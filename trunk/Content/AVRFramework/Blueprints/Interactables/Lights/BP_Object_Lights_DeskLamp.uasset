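; BP_Object_Lights_DeskLamp is a desk lamp light object that extends a parent light Blueprint with an emissive brightness response.
; When InterfaceUpdateLightValue fires, it runs the parent logic, then creates a dynamic material instance on the Root's material index 1.
; It feeds the received percentage into that material's BrightnessEmissive parameter.
; Tick and the construction script only call their parent versions.
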(event `self.ReceiveTick`
  (params (DeltaSeconds :type "Float (single-precision)"))
  (`parent.ReceiveTick` DeltaSeconds))

(event `/Game/AVRFramework/Interface/Interface_Light.Interface_UpdateLightValue`
  (params (Procent :type "Float (single-precision)"))
  (`parent.Interface_UpdateLightValue` Procent)
  (bind _returnvalue (`PrimitiveComponent.CreateDynamicMaterialInstance` (`self.Root`) 1 null "None"))
  (`MaterialInstanceDynamic.SetScalarParameterValue` _returnvalue "BrightnessEmissive" Procent))

(fn `UserConstructionScript`
  (`parent.UserConstructionScript`))