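; Round ceiling light interactable in the AVR framework that adds an emissive-style brightness response to its parent light Blueprint.
; On each interface light-value update it runs the parent logic, then fetches a dynamic material instance from the first material slot of Root.
; It stores that instance and drives its Brightness parameter by linearly mapping the incoming percentage onto the fixture's brightness range.
; All other events and construction defer to the parent.
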(event `self.ReceiveBeginPlay`
  (`parent.ReceiveBeginPlay`))

(event `self.ReceiveTick`
  (params (DeltaSeconds :type "Float (single-precision)"))
  (`parent.ReceiveTick` DeltaSeconds))

(event `self.Interface_UpdateLightValue`
  (params (Procent :type "Float (single-precision)"))
  (`parent.Interface_UpdateLightValue` Procent)
  (bind _returnvalue (`PrimitiveComponent.CreateDynamicMaterialInstance` (`self.Root`) 0 null "None"))
  (set `self.LightMaterial` _returnvalue)
  (`MaterialInstanceDynamic.SetScalarParameterValue` (`self.LightMaterial`) "Brightness" (`KismetMathLibrary.Lerp` 0.0 1.5 Procent)))

(fn `UserConstructionScript`
  (`parent.UserConstructionScript`))