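; BP_Object_Doors is a base door interactable in AVRFramework that opens and closes through interface calls for set, toggle and single triggers.
; A timeline plays or reverses with the open state, feeding a lerped angle-or-distance and progress into MoveDoor.
; MoveDoor is an empty hook, apparently for child doors to implement the motion.
; The construction script applies the initial open state by manipulating the timeline to its start or end.
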(event `self.Interface_SetConstructionOpen`
  (params (Set :type Boolean))
  ;[1 1 1] Handle Open
  (`/Game/AVRFramework/Libraries/MLib_Object_Macros.ManipulateTimeline` (`self.DoorOpenTimeline`) Set))

(event `self.Interface_SetOpen`
  (params (Set :type Boolean))
  ;[1 1 1] Handle Open
  (bind _output_get (set `self.IsOpen` Set))
  (if _output_get
    (bind (_direction _procent) (`Timeline|DoorOpenTimeline` :!label _label)
      (:`Update`
        (`self.MoveDoor` (`KismetMathLibrary.Lerp` 0.0 (`self.AngleOrDistanceToOpen`) _procent) _procent)))
    (else
      (goto _label :!via `Reverse`))))

(event `self.Interface_ToggleOpen`
  ;[1 1 1] Handle Open
  (`self.Interface_SetOpen` (not (`self.IsOpen`))))

(event `/Game/AVRFramework/Interface/Interface_ListenToTrigger.Interface_TriggerSingle`
  (params (Section :type "/Game/AVRFramework/Structs/Struct_Section Structure") (Source :type "Actor Object Reference"))
  ;[1 1 1] Open when being triggered
  (`self.Interface_SetOpen` Section_Set_10_F815F62F4975A2161C6C1E96D17A49FF))

(event `/Game/AVRFramework/Interface/Interface_ListenToTrigger.Interface_TriggerSingleToggle`
  (params (Source :type "Actor Object Reference"))
  ;[1 1 1] Open when being triggered
  (`self.Interface_ToggleOpen`))

(fn `Interface_IsOpen`
  (returns (IsOpen :type Boolean))
  (return (`self.IsOpen`)))

(fn `MoveDoor`
  (params (AngleOrDistance :type "Float (double-precision)") (Procent :type "Float (double-precision)")))

(fn `UserConstructionScript`
  (`parent.UserConstructionScript`)
  (`self.Interface_SetConstructionOpen` (`self.IsOpen`)))