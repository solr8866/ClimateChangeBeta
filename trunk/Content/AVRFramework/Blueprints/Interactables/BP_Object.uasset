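; BP_Object is an interactable object Blueprint in the AVRFramework with animated Appear and Delete events.
; Both events forward to standardAppearLogic, with Appear passing AppearTimeline, its direction and alpha, and one animation for both appearing and deleting.
; AppearTimeline has no play input wired here; its Update and Finished outputs call the logic's Update and Finish.
; BeginPlay, overlap and Tick are disabled stubs.
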(event EventBeginPlay
  (|CallParentFunction) ; This node is disabled and will not be called.\nDrag off pins to build functionality.
)

(event Collision|EventActorBeginOverlap
  (params (OtherActor :type Actor%20Object%20Reference))
  (|CallParentFunction OtherActor) ; This node is disabled and will not be called.\nDrag off pins to build functionality.
)

(event EventTick
  (params (DeltaSeconds :type Float%20%28single-precision%29))
  (|CallParentFunction DeltaSeconds) ; This node is disabled and will not be called.\nDrag off pins to build functionality.
)

(event EventAppear
  (params (AnimToUse :type Enum_DeleteAppearAnim%20Enum :default "NewEnumerator0"))
  (Utilities|StandardAppearLogic (stale _direction) (stale _procent) (Variables|Default|GetAppearTimeline) AnimToUse (stale EventDelete AnimToUse)) ; enters at Appear
)

(event EventDelete
  (params (AnimToUse :type Enum_DeleteAppearAnim%20Enum :default "NewEnumerator0"))
  (Utilities|StandardAppearLogic (stale _direction) (stale _procent) (Variables|Default|GetAppearTimeline) (stale EventAppear AnimToUse) AnimToUse) ; enters at Delete
)

(fn ConstructionScript
  (|CallParentFunction))