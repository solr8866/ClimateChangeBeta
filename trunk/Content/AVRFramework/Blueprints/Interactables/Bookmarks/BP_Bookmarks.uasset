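; BP_Bookmarks is a selectable bookmark interactable in the AVR framework.
; Selection is always allowed, and a press spawns a selection menu at the impact location through CompSelectionMenu.
; Appear and Delete events delegate to shared standardAppearLogic, with Appear passing in AppearTimeline and the requested animation.
; The construction script runs ComponentConstruction to add an arrow component.
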(event EventBeginPlay
  (|CallParentFunction))

(event Collision|EventActorBeginOverlap
  (params (OtherActor :type Actor%20Object%20Reference))
  (|CallParentFunction OtherActor) ; This node is disabled and will not be called.\nDrag off pins to build functionality.
)

(event EventAppear
  (params (AnimToUse :type Enum_DeleteAppearAnim%20Enum :default "NewEnumerator0"))
  ;[1 1 1] Handle Appear
  (Utilities|StandardAppearLogic (stale _direction) (stale _procent) (Variables|Default|GetAppearTimeline) AnimToUse (stale EventDelete AnimToUse)) ; enters at Appear
)

(event EventDelete
  (params (AnimToUse :type Enum_DeleteAppearAnim%20Enum :default "NewEnumerator0"))
  ;[1 1 1] Handle Appear
  (Utilities|StandardAppearLogic (stale _direction) (stale _procent) (Variables|Default|GetAppearTimeline) (stale EventAppear AnimToUse) AnimToUse) ; enters at Delete
)

(event EventTick
  (params (DeltaSeconds :type Float%20%28single-precision%29))
  (|CallParentFunction DeltaSeconds))

(event EventSelectPressed
  (params (Pawn :type BP%20Pawn%20Base%20Object%20Reference) (BaseMotionController :type BP%20Base%20Motion%20Controller%20Object%20Reference) (MotionController :type Motion%20Controller%20Component%20Object%20Reference) (MComp :type BP%20M%20Comp%20Object%20Reference) (ImpactLocation :type Vector :default "0, 0, 0") (ImpactComponent :type Actor%20Component%20Object%20Reference))
  ;[1 1 1] Handle Select
  (Default|SpawnSelectionMenu (Variables|Default|GetComp_SelectionMenu) Pawn ImpactLocation))

(fn ConstructionScript
  (|CallParentFunction)
  (Utilities|ComponentConstruction (stale _returnvalue)
    (:CreateArrow
      (bind _returnvalue (AddComponent|AddArrowComponent false)))))

(fn CanbeSelected
  (return true))