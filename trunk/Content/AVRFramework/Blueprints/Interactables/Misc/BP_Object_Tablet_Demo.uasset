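; Demo tablet interactable for the AVR Framework that plays or pauses content on its tablet screen widget.
; Setting it active through the interface casts the widget component's user widget to Widget_Tablet and calls PlayPause with that state.
; Toggle passes the inverse of IsActive to the set event, though this graph only reads IsActive and never writes it.
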(event `self.ReceiveBeginPlay`
  (`parent.ReceiveBeginPlay`))

(event `self.ReceiveTick`
  (params (DeltaSeconds :type "Float (single-precision)"))
  (`parent.ReceiveTick` DeltaSeconds))

(event `self.Interface_SetActive`
  (params (Set :type Boolean))
  (bind _aswidget_tablet (cast `/Game/AVRFramework/Blueprints/Widgets/Custom/Widget_Tablet` (`WidgetComponent.GetUserWidgetObject` (`self.Widget`))))
  (`/Game/AVRFramework/Blueprints/Widgets/Custom/Widget_Tablet.PlayPause` _aswidget_tablet Set))

(event `self.Interface_ToggleActive`
  (bind _isactive (`self.Interface_IsActive`))
  (`self.Interface_SetActive` (not _isactive)))

(fn `Interface_IsActive`
  (returns (IsActive :type Boolean))
  (return (`self.IsActive`)))

(fn `UserConstructionScript`
  (`parent.UserConstructionScript`))