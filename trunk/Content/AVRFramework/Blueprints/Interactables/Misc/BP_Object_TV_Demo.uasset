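; Demo TV interactable for AVRFramework that plays a looping media source through a Media Player.
; On BeginPlay it opens the TV screen source and, if inactive, pauses it after a short delay.
; Active-state interface functions report, set or toggle its state, playing or pausing the video to match.
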(event `self.ReceiveBeginPlay`
  (bind _mediaplayer (`self.MediaPlayer`))
  (`parent.ReceiveBeginPlay`)
  (`MediaPlayer.OpenSource` _mediaplayer "/Game/AVRFramework/Movies/RVSource_TVScreen.RVSource_TVScreen")
  (`MediaPlayer.SetLooping` _mediaplayer true)
  (bind _isactive (`self.Interface_IsActive`))
  (if (not _isactive)
    (`KismetSystemLibrary.Delay` 3.0)
    (`MediaPlayer.Pause` _mediaplayer)))

(event `self.Interface_SetActive`
  (params (Set :type Boolean))
  (bind _mediaplayer (`self.MediaPlayer`))
  (bind _output_get (set `self.IsActive` Set))
  (if _output_get
    (`MediaPlayer.Play` _mediaplayer)
    (else
      (`MediaPlayer.Pause` _mediaplayer))))

(event `self.Interface_ToggleActive`
  (bind _isactive (`self.Interface_IsActive`))
  (`self.Interface_SetActive` (not _isactive)))

(fn `Interface_IsActive`
  (returns (IsActive :type Boolean))
  (return (`self.IsActive`)))

(fn `UserConstructionScript`
  (`parent.UserConstructionScript`))