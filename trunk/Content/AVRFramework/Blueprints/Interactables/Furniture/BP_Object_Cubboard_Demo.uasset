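; Demo cupboard for the VR framework's interactable furniture, applying one configurable drag type to its child drawers.
; On BeginPlay it casts the child actors of its four Cupboard components to BP_Trigger_Drawer_Example and copies the drag type onto each.
; The construction script writes that drag type into a text label, shown only when tutorial text is enabled.
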(event `self.ReceiveBeginPlay`
  (`parent.ReceiveBeginPlay`)
  (`self.SetChildrenDragType` (`self.Cupboard01`))
  (`self.SetChildrenDragType` (`self.Cupboard02`))
  (`self.SetChildrenDragType` (`self.Cupboard03`))
  (`self.SetChildrenDragType` (`self.Cupboard04`)))

(fn `SetChildrenDragType`
  (params (Childactor :type "ChildActorComponent Object Reference"))
  (bind _asbp_trigger_drawer_example (cast `/Game/AVRFramework/Blueprints/Triggers/Examples/BP_Trigger_Drawer_Example` (`ChildActorComponent.ChildActor` Childactor)))
  (set `/Game/AVRFramework/Blueprints/Triggers/BP_Trigger_Drag.DragType` (`self.ChildenDragType`) _asbp_trigger_drawer_example))

(fn `UserConstructionScript`
  (`parent.UserConstructionScript`)
  (`TextRenderComponent.K2_SetText` (`self.DragType`) (`KismetTextLibrary.Conv_StringToText` (`|GetEnumeratorNameAsString` (`self.ChildenDragType`))))
  (`SceneComponent.SetVisibility` (`self.DragType`) (`self.ShowTutorialText`) false))