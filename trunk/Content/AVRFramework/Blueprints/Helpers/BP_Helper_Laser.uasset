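; VR framework helper that draws a curved laser pointer beam and can be toggled active through interface calls, which show or hide its meshes.
; UpdateLaser bends a runtime spline from the forward direction toward the end point using sine-eased nested lerps, then stretches lazily created spline meshes along it.
; SetLaserColor sets or interpolates color, opacity and beam radii, driving two dynamic materials, the second at reduced opacity.
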(event EventBeginPlay
  (|CallParentFunction)
  ;[1 1 1] Prepare Pointer Spline
  (bind _returnvalue (AddComponent|AddSplineComponent false))
  (bind _output_get (Variables|Default|SetHelperSpline _returnvalue))
  (Spline|ClearSplinePoints _output_get true)
  (bind _returnvalue_2 (Rendering|Material|CreateDynamicMaterialInstance "/Game/AVRFramework/Materials/Framework/Controller/Laser/Mat_Framework_Laser_Solid.Mat_Framework_Laser_Solid" "None" :!class /Script/Engine.KismetMaterialLibrary))
  (Variables|Pointer|SetSplineMaterial00 _returnvalue_2)
  (bind _returnvalue_3 (Rendering|Material|CreateDynamicMaterialInstance "/Game/AVRFramework/Materials/Framework/Controller/Laser/Mat_Framework_Laser_Solid.Mat_Framework_Laser_Solid" "None" :!class /Script/Engine.KismetMaterialLibrary))
  (Variables|Pointer|SetSplineMaterial01 _returnvalue_3))

(event EventTick
  (params (DeltaSeconds :type Float%20%28single-precision%29))
  (|CallParentFunction DeltaSeconds))

(event EventInterfaceSetActive
  (params (Set :type Boolean))
  ;[1 1 1] Handle Activate/Deactivate
  (bind _output_get (Variables|Pointer|SetActive Set))
  (for _array_element (Variables|Pointer|GetSplineMeshes)
    (Rendering|SetVisibility _array_element _output_get false)))

(event EventInterfaceToggleActive
  ;[1 1 1] Handle Activate/Deactivate
  (CallFunction|InterfaceSetActive (not (Variables|Pointer|GetActive))))

(fn ConstructionScript)

(fn UpdateLaser
  (params (StartLocation :type Vector) (EndLocation :type Vector) (ForwardVector :type Vector))
  (bind _helperspline (Variables|Default|GetHelperSpline))
  (LocalVariables|SetLocalStartLocation StartLocation)
  (LocalVariables|SetLocalEndLocations EndLocation)
  (LocalVariables|SetDistance (CallFunction|DistanceBetweenVectors (LocalVariables|GetLocalEndLocations) (LocalVariables|GetLocalStartLocation)))
  (LocalVariables|SetLocalDesiredVector (+ (LocalVariables|GetLocalStartLocation) (* ForwardVector (LocalVariables|GetDistance))))
  (if (== (Spline|GetNumberOfSplinePoints (Variables|Default|GetHelperSpline)) 0)
    (for _index (range 0 (- (Variables|Settings|GetSplinePoints) 1))
      (Spline|AddSplinePoint (Variables|Default|GetHelperSpline) (Math|Vector|MakeVector (Math|Conversions|ToFloat(Integer) _index) 0.0 0.0) "Local" false)))
  (for _index_2 (range 0 (- (Variables|Settings|GetSplinePoints) 2))
    (LocalVariables|SetPointAlpha (|(sin((((x/y)*PI)*0.500000))) (Math|Conversions|ToFloat(Integer) _index_2) (Math|Conversions|ToFloat(Integer) (Variables|Settings|GetSplinePoints)) (Math|Trig|GetPI)))
    (Spline|SetLocationatSplinePoint (Variables|Default|GetHelperSpline) _index_2 (Math|Vector|Lerp(Vector) (Math|Vector|Lerp(Vector) (LocalVariables|GetLocalStartLocation) (LocalVariables|GetLocalDesiredVector) (LocalVariables|GetPointAlpha)) (Math|Vector|Lerp(Vector) (LocalVariables|GetLocalStartLocation) (LocalVariables|GetLocalEndLocations) (LocalVariables|GetPointAlpha)) (LocalVariables|GetPointAlpha)) "Local" false))
  (Spline|SetLocationatSplinePoint (Variables|Default|GetHelperSpline) (- (Variables|Settings|GetSplinePoints) 1) (LocalVariables|GetLocalEndLocations) "Local" true)
  (if (== (Utilities|Array|Length (Variables|Pointer|GetSplineMeshes)) 0)
    (for _index_3 (range 0 (- (Variables|Settings|GetSplinePoints) 1))
      (bind _returnvalue (AddComponent|AddSplineMeshComponent true))
      (Utilities|Array|Add (Variables|Pointer|GetSplineMeshes) _returnvalue)
      (Rendering|Material|SetMaterial _returnvalue 0 (Variables|Pointer|GetSplineMaterial00))
      (Rendering|Material|SetMaterial _returnvalue 1 (Variables|Pointer|GetSplineMaterial01))))
  (for _index_4 (range 0 (- (Variables|Settings|GetSplinePoints) 1))
    (SplineMesh|SetStartScale (Utilities|Array|Get(acopy) (Variables|Pointer|GetSplineMeshes) _index_4) (Variables|Visuals|GetBeamRadiusStart) false :!class /Script/Engine.SplineMeshComponent)
    (SplineMesh|SetEndScale (Utilities|Array|Get(acopy) (Variables|Pointer|GetSplineMeshes) _index_4) (Variables|Visuals|GetBeamRadiusEnd) false :!class /Script/Engine.SplineMeshComponent)
    (SplineMesh|SetStartandEnd (Utilities|Array|Get(acopy) (Variables|Pointer|GetSplineMeshes) _index_4) (.Location (Spline|GetLocationandTangentatSplinePoint _helperspline _index_4 "Local")) (.Tangent (Spline|GetLocationandTangentatSplinePoint _helperspline _index_4 "Local")) (.Location (Spline|GetLocationandTangentatSplinePoint _helperspline (+ _index_4 1) "Local")) (.Tangent (Spline|GetLocationandTangentatSplinePoint _helperspline (+ _index_4 1) "Local")) true :!class /Script/Engine.SplineMeshComponent)
    (Rendering|SetVisibility (Utilities|Array|Get(acopy) (Variables|Pointer|GetSplineMeshes) _index_4) true false)))

(fn SetLaserColor
  (params (InterpolationSpeed :type Float%20%28single-precision%29) (DeltaTime :type Float%20%28single-precision%29) (UseInterpolation :type Boolean) (WantedColor :type Linear%20Color%20Structure) (WantedOpacity :type Float%20%28single-precision%29) (RadiusStart :type Vector%202D%20Structure :default "(X=1.000000,Y=1.000000)") (RadiusEnd :type Vector%202D%20Structure :default "(X=1.000000,Y=1.000000)"))
  (Utilities|FlowControl|Sequence
    (:then_0
      (if UseInterpolation
        (Variables|Visuals|SetLaserOpacity (Math|Interpolation|FInterpTo (Variables|Visuals|GetLaserOpacity) WantedOpacity DeltaTime InterpolationSpeed))
        (LocalVariables|SetLocalColor (Class|KismetMathLibrary|CInterpto (LocalVariables|GetLocalColor) WantedColor DeltaTime InterpolationSpeed))
        (Variables|Visuals|SetBeamRadiusStart (Class|KismetMathLibrary|Vector2DInterpto (Variables|Visuals|GetBeamRadiusStart) RadiusStart DeltaTime InterpolationSpeed))
        (Variables|Visuals|SetBeamRadiusEnd (Class|KismetMathLibrary|Vector2DInterpto (Variables|Visuals|GetBeamRadiusEnd) RadiusEnd DeltaTime InterpolationSpeed))
        (else
          (Variables|Visuals|SetLaserOpacity WantedOpacity)
          (LocalVariables|SetLocalColor WantedColor)
          (Variables|Visuals|SetBeamRadiusStart RadiusStart)
          (Variables|Visuals|SetBeamRadiusEnd RadiusEnd))))
    (:then_1
      (Rendering|Material|SetVectorParameterValue (Variables|Pointer|GetSplineMaterial01) "LaserColor" (LocalVariables|GetLocalColor) :!class /Script/Engine.MaterialInstanceDynamic)
      (Rendering|Material|SetScalarParameterValue (Variables|Pointer|GetSplineMaterial00) "Opacity" (Variables|Visuals|GetLaserOpacity) :!class /Script/Engine.MaterialInstanceDynamic)
      (Rendering|Material|SetScalarParameterValue (Variables|Pointer|GetSplineMaterial01) "Opacity" (* (Variables|Visuals|GetLaserOpacity) 0.4) :!class /Script/Engine.MaterialInstanceDynamic))))

(fn InterfaceIsActive
  (return (Variables|Pointer|GetActive)))