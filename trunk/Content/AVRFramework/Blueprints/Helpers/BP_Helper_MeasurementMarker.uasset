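; Measurement marker helper actor for the AVR framework, which animates in on spawn and can be placed and grabbed.
; Appear and Delete hand off to a standard appear logic component, driven by the AppearTimeline.
; Delete first destroys all attached measurement connections, so they are removed along with the marker.
; IsInMotion reports true until the marker is placed, and afterwards only while a valid actor grabs it.
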(event EventBeginPlay
  (CallFunction|Appear "NewEnumerator1"))

(event EventDelete
  (params (AnimToUse :type Enum_DeleteAppearAnim%20Enum :default "NewEnumerator0"))
  (bind _result (Utilities|Set|ToArray (Variables|Default|GetMeasurementConnections)))
  (CallFunction|DestroyAllChildren _result "NewEnumerator0")
  (Utilities|StandardAppearLogic (stale _direction) (stale _procent) (Variables|Default|GetAppearTimeline) (stale EventAppear AnimToUse) AnimToUse) ; enters at Delete
)

(event EventTick
  (params (DeltaSeconds :type Float%20%28single-precision%29)))

(event EventAppear
  (params (AnimToUse :type Enum_DeleteAppearAnim%20Enum :default "NewEnumerator0"))
  (Utilities|StandardAppearLogic (stale _direction) (stale _procent) (Variables|Default|GetAppearTimeline) AnimToUse (stale EventDelete AnimToUse)) ; enters at Appear
)

(fn ConstructionScript)

(fn IsinMotion
  (if (Variables|Default|GetPlaced)
    (Utilities|IsValid (Variables|/Game/AVRFramework/Blueprints/Components/Actor/Comp_Grab.Comp_Grab_C|GetGrabbingActor (Variables|Default|GetComp_Grab))
      (:Is%20Valid
        (return true))
      (:Is%20Not%20Valid
        (return false)))
    (else
      (return true))))