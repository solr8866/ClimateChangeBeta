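; BP_Helper_Drag is a temporary helper actor in the AVR Framework that relays VR grab events to an assigned object as drag interactions.
; Its Comp_Grab pickup event sends a drag-pressed message to that object, passing the pawn, grabbing actor, controller, component and the helper itself.
; On release it sends a drag-release message if the object is still valid, then destroys itself.
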(event `self.ReceiveTick`
  (params (DeltaSeconds :type "Float (single-precision)"))
  (`parent.ReceiveTick` DeltaSeconds))

(event `self.Comp_Grab.ActorPickedUp`
  (params (GrabbingPawn :type "/Game/AVRFramework/Framework/BP_Pawn_Base Object Reference") (GrabbingActor :type "Actor Object Reference") (GrabbingMotionController :type "/Game/AVRFramework/Blueprints/VR/MotionControllers/BP_BaseMotionController Object Reference") (GrabbingMComp :type "/Game/AVRFramework/Blueprints/VR/MotionComponents/BP_MComp Object Reference"))
  ;[1 1 1] Extends Grabbing Behaviour
  (message `/Game/AVRFramework/Interface/Interface_Draggable.DragPressed` (`self.AssignedObject`) GrabbingPawn GrabbingActor GrabbingMotionController GrabbingMComp self))

(event `self.Comp_Grab.ActorReleased`
  (bind _assignedobject (`self.AssignedObject`))
  ;[1 1 1] Extends Grabbing Behaviour
  (`/Engine/EditorBlueprintResources/StandardMacros.IsValid` _assignedobject
    (:`Is Valid`
      (message `/Game/AVRFramework/Interface/Interface_Draggable.DragRelease` _assignedobject))
    (:`Is Not Valid`
      _))
  (`self.K2_DestroyActor`))

(fn `UserConstructionScript`
  (`parent.UserConstructionScript`))