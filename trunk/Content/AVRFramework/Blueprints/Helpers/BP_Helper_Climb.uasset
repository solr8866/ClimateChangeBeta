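; VR climbing helper actor that moves the grabbing pawn opposite to hand movement while its grab component is held.
; On pickup it notifies the assigned object and opens a gate, letting Tick apply the controller's relative-location delta as an unswept local offset to the pawn.
; Tick auto-releases when the hand strays too far from the assigned object.
; On release it notifies that object and destroys itself.
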(event `self.Comp_Grab.ActorPickedUp`
  (params (GrabbingPawn :type "/Game/AVRFramework/Framework/BP_Pawn_Base Object Reference") (GrabbingActor :type "Actor Object Reference") (GrabbingMotionController :type "/Game/AVRFramework/Blueprints/VR/MotionControllers/BP_BaseMotionController Object Reference") (GrabbingMComp :type "/Game/AVRFramework/Blueprints/VR/MotionComponents/BP_MComp Object Reference"))
  (bind _grabbingmcomp (`/Game/AVRFramework/Blueprints/Components/Actor/Comp_Grab.GrabbingMComp` (`self.Comp_Grab`)))
  (bind _controllercomponent (`/Game/AVRFramework/Blueprints/VR/MotionComponents/BP_MComp.ControllerComponent` _grabbingmcomp))
  (bind _relativelocation (`SceneComponent.RelativeLocation` _controllercomponent))
  ;[1 1 1] Extends Climbing Behaviour
  (message `/Game/AVRFramework/Interface/Interface_Climbable.Interface_ClimbPressed` (`self.AssignedObject`) GrabbingPawn GrabbingMotionController GrabbingMComp self)
  (`|ExecutionSequence`
    (:`then_0`
      (`/Engine/EditorBlueprintResources/StandardMacros.IsValid` _grabbingmcomp :!label _label
        (:`Is Valid`
          (`/Engine/EditorBlueprintResources/StandardMacros.IsValid` _controllercomponent
            (:`Is Valid`
              (set `self.Difference` (- (`self.LastRelativeLocation`) _relativelocation))
              (set `self.LastRelativeLocation` _relativelocation))))))
    (:`then_1`
      (goto _label_2 :!via `Open`))))

(event `self.ReceiveTick`
  (params (DeltaSeconds :type "Float (single-precision)"))
  ;[1 1 1] Extends Climbing Behaviour
  (`parent.ReceiveTick` DeltaSeconds)
  (`|ExecutionSequence`
    (:`then_0`
      (goto _label))
    (:`then_1`
      (`/Engine/EditorBlueprintResources/StandardMacros.Gate` true :!label _label_2
        (:`Exit`
          (`self.K2_AddActorLocalOffset` (`/Game/AVRFramework/Blueprints/Components/Actor/Comp_Grab.GrabbingPawn` (`self.Comp_Grab`)) (`self.Difference`) false false))))
    (:`then_2`
      ;[1 1 1] Auto "Let Go" if the hand is too far away of what he has grabbed
      (if (> (`self.GetDistanceTo` (`self.AssignedObject`) (`/Game/AVRFramework/Blueprints/Components/Actor/Comp_Grab.GrabbingMComp` (`self.Comp_Grab`))) 20.0)
        (message `/Game/AVRFramework/Interface/Interface_GrabbingActor.ReleaseActor` (`/Game/AVRFramework/Blueprints/Components/Actor/Comp_Grab.GrabbingMComp` (`self.Comp_Grab`)) true)))))

(event `self.Comp_Grab.ActorReleased`
  ;[1 1 1] Extends Climbing Behaviour
  (message `/Game/AVRFramework/Interface/Interface_Draggable.DragRelease` (`self.AssignedObject`))
  (`|ExecutionSequence`
    (:`then_0`
      (goto _label_2 :!via `Close`))
    (:`then_1`
      (`self.K2_DestroyActor`))))

(fn `UserConstructionScript`
  (`parent.UserConstructionScript`))