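; Helper actor for the AVR framework that represents a photo shown on a plane and can save it as an image file.
; PrintPicture creates a render target, binds it to a dynamic material on the plane, stores the timecode and returns the target, presumably for a caller to capture into.
; ExportPhoto writes that target to the main game mode's export path as a timecode-named PNG and returns the path.
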(event `self.ReceiveTick`
  (params (DeltaSeconds :type "Float (single-precision)")))

(event `self.ReceiveBeginPlay`)

(fn `ExportPhoto`
  (returns (Path :type String))
  (bind _returnvalue (`KismetStringLibrary.Concat_StrStr` "Screen_" (`TimeManagementBlueprintLibrary.Conv_TimecodeToString` (`TimeManagementBlueprintLibrary.GetTimecode`)) ".png"))
  ;[1 1 1] Export Picture to FilePath defined in the Universal Object
  (bind _asbp_game_mode_main (`/Game/AVRFramework/Libraries/Lib_Core.getMainGameMode` self))
  (bind _exportpath (`/Game/AVRFramework/Framework/BP_GameMode_Main.ExportPath` _asbp_game_mode_main))
  (`KismetRenderingLibrary.ExportRenderTarget` (`self.TextureTarget`) _exportpath _returnvalue)
  (return (`KismetStringLibrary.Concat_StrStr` _exportpath "/" _returnvalue)))

(fn `getPhoto`
  (returns (ReturnValue :type "MaterialInterface Object Reference"))
  (return (`PrimitiveComponent.GetMaterial` (`self.Plane`) 0)))

(fn `PrintPicture`
  (returns (TextureTarget :type "TextureRenderTarget2D Object Reference"))
  (bind _returnvalue (`KismetRenderingLibrary.CreateRenderTarget2D` 800 500 "RTF_RGBA8"))
  (set `self.TextureTarget` _returnvalue)
  ;[1 1 1] Create Photo Instance with the Photo Material
  (bind _returnvalue_2 (`PrimitiveComponent.CreateDynamicMaterialInstance` (`self.Plane`) 0 null "None"))
  (`MaterialInstanceDynamic.SetTextureParameterValue` _returnvalue_2 "Texture" _returnvalue)
  (set `self.Time` (`TimeManagementBlueprintLibrary.GetTimecode`))
  (return _returnvalue))

(fn `UserConstructionScript`)