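; BP_Helper_Group is a helper actor that holds a set of actors as a group and registers itself in the main game state's Groups collection on BeginPlay.
; Its functions remove a member or exchange one for another, adding the new actor only if the old one was removed.
; ShowDebugLines draws temporary debug lines from the helper to each member to visualize the group.
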(event `self.ReceiveBeginPlay`
  (bind _game_state (`/Game/AVRFramework/Libraries/Lib_Core.getMainGameState` self))
  (`BlueprintSetLibrary.Set_Add` (`/Game/AVRFramework/Framework/BP_GameState_Main.Groups` _game_state) self))

(fn `DeleteElementFromGroup`
  (params (OldActor :type "Actor Object Reference"))
  (returns (Success :type Boolean))
  (bind _returnvalue (`BlueprintSetLibrary.Set_Remove` (`self.Group`) OldActor))
  (return _returnvalue))

(fn `ExchangeGroupElement`
  (params (OldActor :type "Actor Object Reference") (NewActor :type "Actor Object Reference"))
  (bind _success (`self.DeleteElementFromGroup` OldActor))
  (if _success
    (`BlueprintSetLibrary.Set_Add` (`self.Group`) NewActor)))

(fn `ShowDebugLines`
  (bind _result (`BlueprintSetLibrary.Set_ToArray` (`self.Group`)))
  (for _array_element _result
    (`KismetSystemLibrary.DrawDebugLine` (`self.K2_GetActorLocation`) (`self.K2_GetActorLocation` _array_element) (struct :`G` 0.290325 :`B` 1.0 :`A` 1.0) 10.0 1.0)))

(fn `UserConstructionScript`)