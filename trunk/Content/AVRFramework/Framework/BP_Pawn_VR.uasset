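; VR player pawn that sets up tracking height per HMD, spawns swappable motion controller actors for each hand and handles player scale.
; Forwards buttons, trigger and grip axes, capacitive touch and thumbstick direction to those controllers.
; Tick also eases the torso mesh toward head yaw.
; An in-development desktop spectator mode switches screen layouts by number key and spawns a non-VR spectator pawn, driven by keyboard and mouse and movable between placed spectator positions.
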(event `Key|MotionController_Left_Trigger`
  (params (Key :type "Key Structure"))
  ;[1 1 1] Forward Inputs to Motion Controller
  (:`Pressed`
    (`self.SetButtonSet` "NewEnumerator0" :!label _label))
  (:`Released`
    (goto _label :!via `LeftReleased`)))

(event `Key|MotionController_Left_FaceButton1` :consume false
  (params (Key :type "Key Structure"))
  ;[1 1 1] Forward Inputs to Motion Controller
  (:`Pressed`
    (`self.SetButtonSet` "NewEnumerator3" :!label _label_2))
  (:`Released`
    (goto _label_2 :!via `LeftReleased`)))

(event `InputAxisKey|OculusTouch_Left_IndexPointing` :consume false
  (params (AxisValue :type "Float (single-precision)"))
  ;[1 1 1] Forward Inputs to Motion Controller
  (bind _controller (`self.GetController` "NewEnumerator0")
    (:`found`
      (`/Game/AVRFramework/Blueprints/VR/MotionControllers/BP_BaseMotionController.TriggerCapTouch` _controller AxisValue))))

(event `InputAxis|LookUp`
  (params (AxisValue :type "Float (single-precision)"))
  ;[1 1 1] Keyboard Inputs For Spectator
  (bind _spectator (`self.Spectator`)
    (:`then`
      (`/Game/AVRFramework/Framework/BP_Pawn_NonVR.LookUp` _spectator AxisValue))
    (:`else`)))

(event `Key|MotionController_Right_Trigger`
  (params (Key :type "Key Structure"))
  ;[1 1 1] Forward Inputs to Motion Controller
  (:`Pressed`
    (goto _label :!via `RightPressed`))
  (:`Released`
    (goto _label :!via `RightReleased`)))

(event `Key|MotionController_Right_FaceButton1` :consume false
  (params (Key :type "Key Structure"))
  ;[1 1 1] Forward Inputs to Motion Controller
  (:`Pressed`
    (goto _label_2 :!via `RightPressed`))
  (:`Released`
    (goto _label_2 :!via `RightReleased`)))

(event `InputAxisKey|OculusTouch_Right_IndexPointing`
  (params (AxisValue :type "Float (single-precision)"))
  ;[1 1 1] Forward Inputs to Motion Controller
  (bind _controller (`self.GetController` "NewEnumerator1")
    (:`found`
      (`/Game/AVRFramework/Blueprints/VR/MotionControllers/BP_BaseMotionController.TriggerCapTouch` _controller AxisValue))))

(event `InputAxis|LookRight`
  (params (AxisValue :type "Float (single-precision)"))
  ;[1 1 1] Keyboard Inputs For Spectator
  (bind _spectator (`self.Spectator`)
    (:`then`
      (`/Game/AVRFramework/Framework/BP_Pawn_NonVR.LookRight` _spectator AxisValue))
    (:`else`)))

(event `Key|MotionController_Left_Grip1`
  (params (Key :type "Key Structure"))
  ;[1 1 1] Forward Inputs to Motion Controller
  (:`Pressed`
    (`self.SetButtonSet` "NewEnumerator2" :!label _label_3))
  (:`Released`
    (goto _label_3 :!via `LeftReleased`)))

(event `Key|MotionController_Left_FaceButton2` :consume false
  (params (Key :type "Key Structure"))
  ;[1 1 1] Forward Inputs to Motion Controller
  (:`Pressed`
    (`self.SetButtonSet` "NewEnumerator4" :!label _label_4))
  (:`Released`
    (goto _label_4 :!via `LeftReleased`)))

(event `InputAxisKey|OculusTouch_Left_ThumbUp` :consume false
  (params (AxisValue :type "Float (single-precision)"))
  ;[1 1 1] Forward Inputs to Motion Controller
  (bind _controller (`self.GetController` "NewEnumerator0")
    (:`found`
      (`/Game/AVRFramework/Blueprints/VR/MotionControllers/BP_BaseMotionController.ThumbCapTouch` _controller AxisValue))))

(event `Key|MotionController_Right_Grip1`
  (params (Key :type "Key Structure"))
  ;[1 1 1] Forward Inputs to Motion Controller
  (:`Pressed`
    (goto _label_3 :!via `RightPressed`))
  (:`Released`
    (goto _label_3 :!via `RightReleased`)))

(event `InputAxis|Right`
  (params (AxisValue :type "Float (single-precision)"))
  ;[1 1 1] Keyboard Inputs For Spectator
  (bind _spectator (`self.Spectator`)
    (:`then`
      (`/Game/AVRFramework/Framework/BP_Pawn_NonVR.MoveRight` _spectator AxisValue))
    (:`else`)))

(event `Key|MotionController_Right_FaceButton2` :consume false
  (params (Key :type "Key Structure"))
  ;[1 1 1] Forward Inputs to Motion Controller
  (:`Pressed`
    (goto _label_4 :!via `RightPressed`))
  (:`Released`
    (goto _label_4 :!via `RightReleased`)))

(event `InputAxisKey|OculusTouch_Right_ThumbUp`
  (params (AxisValue :type "Float (single-precision)"))
  ;[1 1 1] Forward Inputs to Motion Controller
  (bind _controller (`self.GetController` "NewEnumerator1")
    (:`found`
      (`/Game/AVRFramework/Blueprints/VR/MotionControllers/BP_BaseMotionController.ThumbCapTouch` _controller AxisValue))))

(event `Key|MotionController_Left_Thumbstick` :consume false
  (params (Key :type "Key Structure"))
  ;[1 1 1] Forward Inputs to Motion Controller
  (:`Pressed`
    (`self.SetButtonSet` "NewEnumerator7" :!label _label_5))
  (:`Released`
    (goto _label_5 :!via `LeftReleased`)))

(event `InputAxis|Forward`
  (params (AxisValue :type "Float (single-precision)"))
  ;[1 1 1] Keyboard Inputs For Spectator
  (bind _spectator (`self.Spectator`)
    (:`then`
      (`/Game/AVRFramework/Framework/BP_Pawn_NonVR.MoveForward` _spectator AxisValue))
    (:`else`)))

(event `Key|MotionController_Left_FaceButton3` :consume false
  (params (Key :type "Key Structure"))
  ;[1 1 1] Forward Inputs to Motion Controller
  (:`Pressed`
    (`self.SetButtonSet` "NewEnumerator5" :!label _label_6))
  (:`Released`
    (goto _label_6 :!via `LeftReleased`)))

(event `self.ReceiveBeginPlay`
  ;[1 1 1] Setup Pawn VR
  (set `self.PlayerSize` (`HeadMountedDisplayFunctionLibrary.GetWorldToMetersScale`))
  (`|ExecutionSequence`
    (:`then_0`
      (switch `name` (`HeadMountedDisplayFunctionLibrary.GetHMDDeviceName`)
        (:`OculusHMD`
          (set `self.HMD` "NewEnumerator1"))
        (:`SteamVR`
          (set `self.HMD` "NewEnumerator0"))
        (:`PSVR`
          (set `self.HMD` "NewEnumerator2"))))
    (:`then_1`
      (`self.SetupHeight` (`self.PlayerHeight`))
      (if (`self.PausePawn`)
        (`self.SwitchControllers` "/Game/AVRFramework/Blueprints/VR/MotionControllers/BP_MotionController_Controller_Pause.BP_MotionController_Controller_Pause_C" "/Game/AVRFramework/Blueprints/VR/MotionControllers/BP_MotionController_Controller_Pause.BP_MotionController_Controller_Pause_C")
        (else
          (bind _infocontrols (`/Game/AVRFramework/Libraries/Lib_Core.getInfoControls` self))
          (bind (_controllerset_leftcontroller _controllerset_rightcontroller) (break `/Game/AVRFramework/Structs/Struct_ControllerSet` (`/Game/AVRFramework/Blueprints/Info/BP_Info_Controls.ControllerSet` _infocontrols)))
          (`self.SwitchControllers` _controllerset_leftcontroller _controllerset_rightcontroller))))))

(event `InputAxisKey|MotionController_Left_Grip1Axis` :consume false
  (params (AxisValue :type "Float (single-precision)"))
  ;[1 1 1] Forward Inputs to Motion Controller
  (bind _controller (`self.GetController` "NewEnumerator0")
    (:`found`
      (`/Game/AVRFramework/Blueprints/VR/MotionControllers/BP_BaseMotionController.GribAxis` _controller AxisValue))))

(event `Key|MotionController_Right_Thumbstick` :consume false
  (params (Key :type "Key Structure"))
  ;[1 1 1] Forward Inputs to Motion Controller
  (:`Pressed`
    (goto _label_5 :!via `RightPressed`))
  (:`Released`
    (goto _label_5 :!via `RightReleased`)))

(event `InputAxis|Up`
  (params (AxisValue :type "Float (single-precision)"))
  ;[1 1 1] Keyboard Inputs For Spectator
  (bind _spectator (`self.Spectator`)
    (:`then`
      (`/Game/AVRFramework/Framework/BP_Pawn_NonVR.MoveUp` _spectator AxisValue))
    (:`else`)))

(event `Key|MotionController_Right_FaceButton3` :consume false
  (params (Key :type "Key Structure"))
  ;[1 1 1] Forward Inputs to Motion Controller
  (:`Pressed`
    (goto _label_6 :!via `RightPressed`))
  (:`Released`
    (goto _label_6 :!via `RightReleased`)))

(event `Key|MotionController_Left_Shoulder`
  (params (Key :type "Key Structure"))
  ;[1 1 1] Forward Inputs to Motion Controller
  (:`Pressed`
    (`self.SetButtonSet` "NewEnumerator8" :!label _label_7))
  (:`Released`
    (goto _label_7 :!via `LeftReleased`)))

(event `InputAxisKey|MotionController_Right_Grip1Axis`
  (params (AxisValue :type "Float (single-precision)"))
  ;[1 1 1] Forward Inputs to Motion Controller
  (bind _controller (`self.GetController` "NewEnumerator1")
    (:`found`
      (`/Game/AVRFramework/Blueprints/VR/MotionControllers/BP_BaseMotionController.GribAxis` _controller AxisValue))))

(event `Key|MotionController_Left_FaceButton4` :consume false
  (params (Key :type "Key Structure"))
  ;[1 1 1] Forward Inputs to Motion Controller
  (:`Pressed`
    (`self.SetButtonSet` "NewEnumerator6" :!label _label_8))
  (:`Released`
    (goto _label_8 :!via `LeftReleased`)))

(event `Key|SpaceBar`
  (params (Key :type "Key Structure"))
  ;[1 1 1] Keyboard Inputs For Spectator
  (:`Pressed`
    (bind _spectator (`self.Spectator`)
      (:`then`
        (`/Game/AVRFramework/Framework/BP_Pawn_NonVR.SetJump` _spectator true))
      (:`else`)))
  (:`Released`
    (bind _spectator_2 (`self.Spectator`)
      (:`then`
        (`/Game/AVRFramework/Framework/BP_Pawn_NonVR.SetJump` _spectator_2 false))
      (:`else`))))

(event `Key|MotionController_Right_Shoulder`
  (params (Key :type "Key Structure"))
  ;[1 1 1] Forward Inputs to Motion Controller
  (:`Pressed`
    (goto _label_7 :!via `RightPressed`))
  (:`Released`
    (goto _label_7 :!via `RightReleased`)))

(event `SetupHeight`
  (params (Height :type "Float (double-precision)" :default 180.0))
  ;[1 1 1] Setup Pawn VR
  ;;[1 1 1] Setup Hight and Tracking Origin
  (switch `/Game/AVRFramework/Enums/Enum_HMD` (`self.HMD`)
    (:`NewEnumerator0`
      (`HeadMountedDisplayFunctionLibrary.SetTrackingOrigin` "Floor" :!label _label_9))
    (:`NewEnumerator1`
      (goto _label_9))
    (:`NewEnumerator2`
      (`HeadMountedDisplayFunctionLibrary.SetTrackingOrigin` "Eye")
      (`SceneComponent.K2_AddLocalOffset` (`self.VRHandle`) (`KismetMathLibrary.MakeVector` 0.0 0.0 Height) false false))))

(event `InputAxisKey|MotionController_Left_TriggerAxis`
  (params (AxisValue :type "Float (single-precision)"))
  ;[1 1 1] Forward Inputs to Motion Controller
  (bind _controller (`self.GetController` "NewEnumerator0")
    (:`found`
      (`/Game/AVRFramework/Blueprints/VR/MotionControllers/BP_BaseMotionController.TriggerAxis` _controller AxisValue))))

(event `Key|MotionController_Right_FaceButton4` :consume false
  (params (Key :type "Key Structure"))
  ;[1 1 1] Forward Inputs to Motion Controller
  (:`Pressed`
    (goto _label_8 :!via `RightPressed`))
  (:`Released`
    (goto _label_8 :!via `RightReleased`)))

(event `InputAxisKey|MotionController_Right_TriggerAxis`
  (params (AxisValue :type "Float (single-precision)"))
  ;[1 1 1] Forward Inputs to Motion Controller
  (bind _controller (`self.GetController` "NewEnumerator1")
    (:`found`
      (`/Game/AVRFramework/Blueprints/VR/MotionControllers/BP_BaseMotionController.TriggerAxis` _controller AxisValue))))

(event `Key|RightMouseButton`
  (params (Key :type "Key Structure"))
  ;[1 1 1] Keyboard Inputs For Spectator
  (:`Pressed`
    (bind _spectator (`self.Spectator`)
      (:`then`
        (`/Game/AVRFramework/Framework/BP_Pawn_NonVR.ToggleMouse` _spectator))
      (:`else`))))

(event `self.SetPlayerSize`
  (params (Size :type "Float (single-precision)"))
  ;[1 1 1] Setup Pawn VR
  ;;[1 1 1] Set Player Size
  (`parent.SetPlayerSize` Size)
  (`HeadMountedDisplayFunctionLibrary.SetWorldToMetersScale` (`self.PlayerSize`))
  (bind _controller (`self.GetController` "NewEnumerator1")
    (:`found`
      (bind _controller_2 (`self.GetController` "NewEnumerator0")
        (:`found`
          (`/Game/AVRFramework/Blueprints/VR/MotionControllers/BP_BaseMotionController.SetPLayerSize` _controller (/ (`self.PlayerSize`) 100.0))
          (`/Game/AVRFramework/Blueprints/VR/MotionControllers/BP_BaseMotionController.SetPLayerSize` _controller_2 (/ (`self.PlayerSize`) 100.0)))))))

(event `Key|LeftMouseButton`
  (params (Key :type "Key Structure"))
  ;[1 1 1] Keyboard Inputs For Spectator
  (:`Pressed`
    (bind _spectator (`self.Spectator`)
      (:`then`
        (`/Game/AVRFramework/Framework/BP_Pawn_NonVR.Trigger` _spectator true))
      (:`else`)))
  (:`Released`
    (bind _spectator_2 (`self.Spectator`)
      (:`then`
        (`/Game/AVRFramework/Framework/BP_Pawn_NonVR.Trigger` _spectator_2 false))
      (:`else`))))

(event `InputAction|Sprint`
  (params (Key :type "Key Structure"))
  ;[1 1 1] Keyboard Inputs For Spectator
  (:`Pressed`
    (bind _spectator (`self.Spectator`)
      (:`then`
        (`/Game/AVRFramework/Framework/BP_Pawn_NonVR.SetSprint` _spectator true))
      (:`else`)))
  (:`Released`
    (bind _spectator_2 (`self.Spectator`)
      (:`then`
        (`/Game/AVRFramework/Framework/BP_Pawn_NonVR.SetSprint` _spectator_2 false))
      (:`else`))))

(event `SwitchControllers`
  (params (LeftController :type "/Game/AVRFramework/Blueprints/VR/MotionControllers/BP_BaseMotionController Class Reference") (RightController :type "/Game/AVRFramework/Blueprints/VR/MotionControllers/BP_BaseMotionController Class Reference"))
  ;[1 1 1] Setup Pawn VR
  ;;[1 1 1] Setup VR Controllers
  (`self.SetUpHand` LeftController)
  (`self.SetUpHand` RightController "NewEnumerator1")
  (`self.SetPlayerSize` (`self.PlayerSize`)))

(event `self.ReceiveTick`
  (params (DeltaSeconds :type "Float (single-precision)"))
  (bind _returnvalue (`self.GetInputAxisKeyValue`))
  (bind _returnvalue_2 (`self.GetInputAxisKeyValue`))
  (bind _returnvalue_3 (`self.GetInputAxisKeyValue`))
  (bind _returnvalue_4 (`self.GetInputAxisKeyValue`))
  (bind _smesh_framework_torso (`self.SMesh_Framework_Torso`))
  (bind (_returnvalue_roll _returnvalue_pitch _returnvalue_yaw) (`KismetMathLibrary.BreakRotator` (`SceneComponent.K2_GetComponentRotation` (`self.SMesh_Framework_Head`))))
  (bind _returnvalue_5 (* _returnvalue_3 -1.0))
  (bind _returnvalue_6 (* _returnvalue -1.0))
  (bind (_outrotation _outrotationnooffset) (`self.CalculateRotation` _returnvalue_6 _returnvalue_2))
  (bind (_outrotation_2 _outrotationnooffset_2) (`self.CalculateRotation` _returnvalue_5 _returnvalue_4))
  ;[1 1 1] Forward Thumbstick Information to Motion Controllers
  (`parent.ReceiveTick` DeltaSeconds)
  (`|ExecutionSequence`
    (:`then_0`
      (bind _controller (`self.GetController` "NewEnumerator0")
        (:`found`
          (`/Game/AVRFramework/Blueprints/VR/MotionControllers/BP_BaseMotionController.SetThumbstickRotation` _controller _outrotation_2 _outrotationnooffset_2 _returnvalue_5 _returnvalue_4)
          (if (or (> (`KismetMathLibrary.Abs` _returnvalue_3) 0.3) (> (`KismetMathLibrary.Abs` _returnvalue_4) 0.3))
            (`/Engine/EditorBlueprintResources/StandardMacros.DoOnce` false :!label _label_10
              (:`Completed`
                (`|ExecutionSequence`
                  (:`then_0`
                    (`self.SetButtonSet` "NewEnumerator9" :!label _label_11))
                  (:`then_1`
                    (goto _label_12 :!via `Reset`)))))
            (else
              (`/Engine/EditorBlueprintResources/StandardMacros.DoOnce` true :!label _label_12
                (:`Completed`
                  (`|ExecutionSequence`
                    (:`then_0`
                      (goto _label_11 :!via `LeftReleased`))
                    (:`then_1`
                      (goto _label_10 :!via `Reset`))))))))))
    (:`then_1`
      (bind _controller_2 (`self.GetController` "NewEnumerator1")
        (:`found`
          (`/Game/AVRFramework/Blueprints/VR/MotionControllers/BP_BaseMotionController.SetThumbstickRotation` _controller_2 _outrotation _outrotationnooffset _returnvalue_6 _returnvalue_2)
          (if (or (> (`KismetMathLibrary.Abs` _returnvalue) 0.3) (> (`KismetMathLibrary.Abs` _returnvalue_2) 0.3))
            (`/Engine/EditorBlueprintResources/StandardMacros.DoOnce` false :!label _label_13
              (:`Completed`
                (`|ExecutionSequence`
                  (:`then_0`
                    (goto _label_11 :!via `RightPressed`))
                  (:`then_1`
                    (goto _label_14 :!via `Reset`)))))
            (else
              (`/Engine/EditorBlueprintResources/StandardMacros.DoOnce` true :!label _label_14
                (:`Completed`
                  (`|ExecutionSequence`
                    (:`then_0`
                      (goto _label_11 :!via `RightReleased`))
                    (:`then_1`
                      (goto _label_13 :!via `Reset`))))))))))
    (:`then_2`
      ;[1 1 1] SetBody Position
      (`SceneComponent.K2_SetWorldRotation` _smesh_framework_torso (`KismetMathLibrary.RInterpTo` (`SceneComponent.K2_GetComponentRotation` _smesh_framework_torso) (`KismetMathLibrary.MakeRotator` 0.0 0.0 _returnvalue_yaw) DeltaSeconds 2.0) false false))))

(event `InputAxis|Zoom`
  (params (AxisValue :type "Float (single-precision)"))
  ;[1 1 1] Keyboard Inputs For Spectator
  (bind _spectator (`self.Spectator`)
    (:`then`
      (`/Game/AVRFramework/Framework/BP_Pawn_NonVR.Zoom` _spectator AxisValue))
    (:`else`)))

(event `/Game/AVRFramework/Interface/Interface_Deleteable.Delete`
  (params (AnimToUse :type "/Game/AVRFramework/Enums/Enum_DeleteAppearAnim Enum" :default "NewEnumerator0"))
  ;[1 1 1] Delete Pawn
  (bind _values (`BlueprintMapLibrary.Map_Values` (`self.Controllers`)))
  (`/Game/AVRFramework/Libraries/MLib_Actor_Macros.DeleteActorsAndWait` _values
    (:`AllGone`
      (`parent.Delete` "NewEnumerator0"))))

(event `Key|One`
  (params (Key :type "Key Structure"))
  ;[1 1 1] Spectator Mode, Still in Development
  (:`Pressed`
    (`self.SetSpectatorMode` 1)))

(event `Key|NumPadZero`
  (params (Key :type "Key Structure"))
  ;[1 1 1] Spectator Mode, Still in Development
  (:`Pressed`
    (`self.MoveSpectatorToPositionWithIndex` 0)))

(event `self.ReceivePossessed`
  (params (NewController :type "Controller Object Reference"))
  ;[1 1 1] Spectator Mode, Still in Development
)

(event `RotateThroughControllers`
  (bind _array (`|MakeArray` "/Game/AVRFramework/Blueprints/VR/MotionControllers/BP_MotionController_Controller_Laser.BP_MotionController_Controller_Laser_C" "/Game/AVRFramework/Blueprints/VR/MotionControllers/BP_MotionController_Controller_Laser_Single.BP_MotionController_Controller_Laser_Single_C" "/Game/AVRFramework/Blueprints/VR/MotionControllers/BP_MotionController_Controller_Pointer.BP_MotionController_Controller_Pointer_C" "/Game/AVRFramework/Blueprints/VR/MotionControllers/BP_MotionController_Hands.BP_MotionController_Hands_C" "/Game/AVRFramework/Blueprints/VR/MotionControllers/BP_MotionController_HandWithWatch.BP_MotionController_HandWithWatch_C" :!type "/Game/AVRFramework/Blueprints/VR/MotionControllers/BP_BaseMotionController Class Reference"))
  ;[1 1 1] Switch between Controller Modi
  (bind _controller (`self.GetController` "NewEnumerator0")
    (:`found`
      (bind _output (`|GetArrayItem` _array (`/Game/AVRFramework/Libraries/FLib_Utility.IncrementIntWithModulo` (`KismetArrayLibrary.Array_Find` _array (`GameplayStatics.GetObjectClass` _controller)) (`KismetArrayLibrary.Array_Length` _array))))
      (`self.SwitchControllers` _output _output))))

(event `Key|Two`
  (params (Key :type "Key Structure"))
  ;[1 1 1] Spectator Mode, Still in Development
  (:`Pressed`
    (`self.SetSpectatorMode` 2)))

(event `Key|NumPadOne`
  (params (Key :type "Key Structure"))
  ;[1 1 1] Spectator Mode, Still in Development
  (:`Pressed`
    (`self.MoveSpectatorToPositionWithIndex` 1)))

(event `Key|Three`
  (params (Key :type "Key Structure"))
  ;[1 1 1] Spectator Mode, Still in Development
  (:`Pressed`
    (`self.SetSpectatorMode` 3)))

(event `Key|NumPadTwo`
  (params (Key :type "Key Structure"))
  ;[1 1 1] Spectator Mode, Still in Development
  (:`Pressed`
    (`self.MoveSpectatorToPositionWithIndex` 2)))

(event `Key|Four`
  (params (Key :type "Key Structure"))
  ;[1 1 1] Spectator Mode, Still in Development
  (:`Pressed`
    (`self.SetSpectatorMode` 4)))

(event `Key|NumPadThree`
  (params (Key :type "Key Structure"))
  ;[1 1 1] Spectator Mode, Still in Development
  (:`Pressed`
    (`self.MoveSpectatorToPositionWithIndex` 3)))

(event `Key|NumPadFour`
  (params (Key :type "Key Structure"))
  ;[1 1 1] Spectator Mode, Still in Development
  (:`Pressed`
    (`self.MoveSpectatorToPositionWithIndex` 4)))

(event `SetSpectatorMode`
  (params (Mode :type Integer))
  (bind _spectator (`self.Spectator`))
  (bind _spectator_2 (`self.Spectator`))
  ;[1 1 1] Spectator Mode, Still in Development
  (switch `int` Mode
    (:`1`
      (`/Engine/EditorBlueprintResources/StandardMacros.IsValid` _spectator_2
        (:`Is Valid`
          (`self.K2_DestroyActor` _spectator_2))
        (:`Is Not Valid`
          _))
      (`HeadMountedDisplayFunctionLibrary.SetSpectatorScreenMode` "SingleEyeCroppedToFill"))
    (:`2`
      (`/Engine/EditorBlueprintResources/StandardMacros.IsValid` _spectator
        (:`Is Valid`
          (`self.K2_DestroyActor` _spectator))
        (:`Is Not Valid`
          _))
      (`HeadMountedDisplayFunctionLibrary.SetSpectatorScreenMode` "Texture")
      (`/Engine/EditorBlueprintResources/StandardMacros.IsValid` (`self.Spectator`) :!label _label_15
        (:`Is Not Valid`
          (bind _spectatorposition (`self.GetBestSpectatorPosition`))
          (`/Engine/EditorBlueprintResources/StandardMacros.IsValid` _spectatorposition
            (:`Is Valid`
              (bind _asbp_player_controller_main (cast `/Game/AVRFramework/Framework/BP_PlayerController_Main` (`self.GetController`)))
              (bind _returnvalue (`|SpawnActorFromClass` "/Game/AVRFramework/Framework/BP_Pawn_NonVR_Spectator.BP_Pawn_NonVR_Spectator_C" (`self.GetTransform` _spectatorposition) "Undefined" "OverrideRootScale" null _asbp_player_controller_main 30.0 false null))
              (bind _output_get (set `self.Spectator` _returnvalue))
              (`/Game/AVRFramework/Framework/BP_Pawn_NonVR.Initiate` _output_get _asbp_player_controller_main))))))
    (:`3`
      (`HeadMountedDisplayFunctionLibrary.SetSpectatorScreenMode` "TexturePlusEye")
      (`HeadMountedDisplayFunctionLibrary.SetSpectatorScreenModeTexturePlusEyeLayout` (0.7 0.02) (0.98 0.4) (0.0 0.0) (1.0 1.0) false)
      (goto _label_15))
    (:`4`
      (`HeadMountedDisplayFunctionLibrary.SetSpectatorScreenMode` "TexturePlusEye")
      (`HeadMountedDisplayFunctionLibrary.SetSpectatorScreenModeTexturePlusEyeLayout` (0.0 0.0) (1.0 1.0) (0.7 0.02) (0.98 0.4))
      (goto _label_15))))

(event `Key|NumPadFive`
  (params (Key :type "Key Structure"))
  ;[1 1 1] Spectator Mode, Still in Development
  (:`Pressed`
    (`self.MoveSpectatorToPositionWithIndex` 5)))

(event `Key|NumPadSix`
  (params (Key :type "Key Structure"))
  ;[1 1 1] Spectator Mode, Still in Development
  (:`Pressed`
    (`self.MoveSpectatorToPositionWithIndex` 6)))

(event `Key|Escape`
  (params (Key :type "Key Structure"))
  ;[1 1 1] Quit Game on Escape
  (:`Released`
    (`KismetSystemLibrary.QuitGame` null "Quit")))

(event `Key|NumPadSeven`
  (params (Key :type "Key Structure"))
  ;[1 1 1] Spectator Mode, Still in Development
  (:`Pressed`
    (`self.MoveSpectatorToPositionWithIndex` 7)))

(event `Key|NumPadEight`
  (params (Key :type "Key Structure"))
  ;[1 1 1] Spectator Mode, Still in Development
  (:`Pressed`
    (`self.MoveSpectatorToPositionWithIndex` 8)))

(event `Key|NumPadNine`
  (params (Key :type "Key Structure"))
  ;[1 1 1] Spectator Mode, Still in Development
  (:`Pressed`
    (`self.MoveSpectatorToPositionWithIndex` 9)))

(fn `CalculateRotation`
  (params (Up :type "Float (double-precision)") (Right :type "Float (double-precision)"))
  (returns (OutRotation :type "Rotator Structure") (OutRotationNoOffset :type "Rotator Structure"))
  (bind _returnvalue (`KismetMathLibrary.Normal` (`KismetMathLibrary.MakeVector` Up Right)))
  (return (`KismetMathLibrary.Conv_VectorToRotator` (`KismetMathLibrary.GreaterGreater_VectorRotator` _returnvalue (`KismetMathLibrary.MakeRotator` 0.0 0.0 (.yaw (`self.K2_GetActorRotation`))))) (`KismetMathLibrary.Conv_VectorToRotator` _returnvalue)))

(fn `GetAllAttachedActors`
  (returns (AttachedActors :type "Set of Actor Object Reference"))
  (locals (Return :type "Set of Actor Object Reference"))
  (`|ExecutionSequence`
    (:`then_0`
      (bind _controller (`self.GetController` "NewEnumerator0")
        (:`found`
          (bind _actors (`/Game/AVRFramework/Blueprints/VR/MotionControllers/BP_BaseMotionController.getAllAttachedActors` _controller))
          (bind _result (`BlueprintSetLibrary.Set_Union` (`local.Return`) _actors))
          (set `local.Return` _result)
          (`BlueprintSetLibrary.Set_Add` (`local.Return`) _controller))))
    (:`then_1`
      (bind _controller_2 (`self.GetController` "NewEnumerator1")
        (:`found`
          (bind _actors_2 (`/Game/AVRFramework/Blueprints/VR/MotionControllers/BP_BaseMotionController.getAllAttachedActors` _controller_2))
          (bind _result_2 (`BlueprintSetLibrary.Set_Union` (`local.Return`) _actors_2))
          (set `local.Return` _result_2)
          (`BlueprintSetLibrary.Set_Add` (`local.Return`) _controller_2))))
    (:`then_2`
      (bind _result_3 (`BlueprintSetLibrary.Set_Union` (`/Game/AVRFramework/Blueprints/Components/Actor/Comp_Attach.AttachedActorSet` (`self.Comp_Attach`)) (`local.Return`)))
      (set `local.Return` _result_3))
    (:`then_3`
      (return (`local.Return`)))))

(fn `GetBestSpectatorPosition`
  (returns (SpectatorPosition :type "/Game/AVRFramework/Blueprints/Navigation/BP_SpectatorPosition Object Reference"))
  (locals (DefaultSpectator :type "/Game/AVRFramework/Blueprints/Navigation/BP_SpectatorPosition Object Reference"))
  (bind _outactors (`GameplayStatics.GetAllActorsOfClass` "/Game/AVRFramework/Blueprints/Navigation/BP_SpectatorPosition.BP_SpectatorPosition_C"))
  (for _array_element _outactors
    (if (== (`/Game/AVRFramework/Blueprints/Navigation/BP_SpectatorPosition.Index` _array_element) 1)
      (return _array_element)
      (elif (`/Game/AVRFramework/Blueprints/Navigation/BP_SpectatorPosition.DefaultSpectatorPosition` _array_element)
        (set `local.DefaultSpectator` _array_element))))
  (return (`local.DefaultSpectator`)))

(fn `GetCameraComponent`
  (returns (Camera :type "CameraComponent Object Reference"))
  (return (`self.Camera`)))

(fn `GetSpectatorPositionFromIndex`
  (params (Index :type Integer))
  (returns (SpectatorPosition :type "/Game/AVRFramework/Blueprints/Navigation/BP_SpectatorPosition Object Reference"))
  (locals (DefaultSpectator :type "/Game/AVRFramework/Blueprints/Navigation/BP_SpectatorPosition Object Reference"))
  (bind _outactors (`GameplayStatics.GetAllActorsOfClass` "/Game/AVRFramework/Blueprints/Navigation/BP_SpectatorPosition.BP_SpectatorPosition_C"))
  (for _array_element _outactors
    (if (== (`/Game/AVRFramework/Blueprints/Navigation/BP_SpectatorPosition.Index` _array_element) Index)
      (return _array_element)))
  (`/Game/AVRFramework/Libraries/Lib_Core.ErrorMessage` self "Spectator Position Not Found")
  (return null))

(fn `GetWorldScaleFactor`
  (returns (`Out ScaleFactor` :type "Float (double-precision)"))
  (return (/ (`HeadMountedDisplayFunctionLibrary.GetWorldToMetersScale`) 100.0)))

(fn `RemoveController`
  (params (BaseMotionController :type "/Game/AVRFramework/Blueprints/VR/MotionControllers/BP_BaseMotionController Object Reference"))
  (`/Engine/EditorBlueprintResources/StandardMacros.IsValid` BaseMotionController
    (:`Is Valid`
      (`/Game/AVRFramework/Blueprints/VR/MotionControllers/BP_BaseMotionController.Delete` BaseMotionController "NewEnumerator0"))))

(fn `SetUpHand`
  (params (MotionControllerClass :type "/Game/AVRFramework/Blueprints/VR/MotionControllers/BP_BaseMotionController Class Reference") (Side :type "/Game/AVRFramework/Enums/Enum_Side Enum" :default "NewEnumerator0"))
  (bind _controller (`self.GetController` Side)
    (:`found`
      (`/Game/AVRFramework/Blueprints/VR/MotionControllers/BP_BaseMotionController.Delete` _controller "NewEnumerator0"))
    (:`NotFound`
      _))
  (bind _returnvalue (`|SpawnActorFromClass` (select `bool` (`KismetSystemLibrary.IsValidClass` MotionControllerClass) :`false` "/Game/AVRFramework/Blueprints/VR/MotionControllers/BP_MotionController_Controller_Pause.BP_MotionController_Controller_Pause_C" :`true` MotionControllerClass) (`KismetMathLibrary.MakeTransform` (0.0 0.0 0.0)) "AlwaysSpawn" "OverrideRootScale" self self (`self.HMD`) Side null))
  (`self.K2_AttachToComponent` _returnvalue (`self.VRHandle`) "None" "SnapToTarget" "SnapToTarget" "SnapToTarget" false)
  (`BlueprintMapLibrary.Map_Add` (`self.Controllers`) Side _returnvalue))

(fn `UserConstructionScript`)